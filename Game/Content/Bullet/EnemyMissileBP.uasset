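; Enemy missile that flies in an arc at the player.
; BeginPlay captures positions and scales a timeline by distance over speed, lerping with a height curve toward the player's live X and initial Y/Z.
; Tick refreshes that X, sets rotation and destroys the missile once the player's X reaches or exceeds its own.
; Guard overlaps drain guard energy and destroy it; guarding-player overlaps play Bounce, while untagged overlaps stop it.
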(event `self.ReceiveBeginPlay`
  (bind (_playerpos_x _playerpos_y _playerpos_z) (`KismetMathLibrary.BreakVector` (`self.PlayerPos`)))
  (bind _startpos_x (`KismetMathLibrary.BreakVector` (`self.StartPos`)))
  (bind _playerpos_x_2 (`KismetMathLibrary.BreakVector` (`self.PlayerPos`)))
  (bind _temppos_x (`KismetMathLibrary.BreakVector` (`self.TempPos`)))
  (bind (_startpos_x_2 _startpos_y _startpos_z) (`KismetMathLibrary.BreakVector` (`self.StartPos`)))
  (bind _asplayer_chara_bp (cast `/Game/BP/PlayerCharaBP` (`GameplayStatics.GetPlayerPawn` 0)))
  (bind (_returnvalue_x _returnvalue_y _returnvalue_z) (`KismetMathLibrary.BreakVector` (`self.K2_GetActorLocation` _asplayer_chara_bp)))
  (set `self.PlayerPos` (`KismetMathLibrary.MakeVector` (- _returnvalue_x 10.0) _returnvalue_y _returnvalue_z))
  (set `self.StartPos` (`self.K2_GetActorLocation`))
  (set `self.FlyTime` (/ (- _startpos_x _playerpos_x_2) (`self.BulletSpeed`)))
  (`TimelineComponent.SetPlayRate` (`self.Fly_TimeLine`) (/ 5.0 (`self.FlyTime`)))
  (bind (_direction _fly_value _up_down_value) (`Timeline|Fly_TimeLine`)
    (:`Update`
      (bind _returnvalue (* _up_down_value (`self.MaxHeight`)))
      (`self.K2_SetActorLocation` (`KismetMathLibrary.VLerp` (`KismetMathLibrary.MakeVector` _startpos_x_2 _startpos_y (+ _returnvalue _startpos_z)) (`KismetMathLibrary.MakeVector` _temppos_x _playerpos_y (+ _returnvalue _playerpos_z)) _fly_value)))))

(event `self.ReceiveActorBeginOverlap`
  (params (OtherActor :type "Actor Object Reference"))
  (if (`self.ActorHasTag` OtherActor "Guard")
    (bind _asplayer_chara_bp (cast `/Game/BP/PlayerCharaBP` (`GameplayStatics.GetPlayerPawn` 0)))
    (set `PlayerChara.GuardEnergy` (- (`PlayerChara.GuardEnergy` _asplayer_chara_bp) 20.0) _asplayer_chara_bp)
    (`self.K2_DestroyActor`)
    (elif (`self.ActorHasTag` OtherActor "Player")
      (bind _asplayer_chara_bp_2 (cast `/Game/BP/PlayerCharaBP` (`GameplayStatics.GetPlayerPawn` 0)))
      (if (`PlayerChara.isGuarding` _asplayer_chara_bp_2)
        (`AudioComponent.Play` (`self.Bounce`) 0.0))
      (else
        (`AudioComponent.Stop` (`self.Bounce`))))))

(event `self.ReceiveTick`
  (params (DeltaSeconds :type "Float (single-precision)"))
  (bind _returnvalue_x (`KismetMathLibrary.BreakVector` (`self.K2_GetActorLocation`)))
  (bind (_playerpos_x _playerpos_y _playerpos_z) (`KismetMathLibrary.BreakVector` (`self.PlayerPos`)))
  (bind _temppos_x (`KismetMathLibrary.BreakVector` (`self.TempPos`)))
  (bind _temppos_x_2 (`KismetMathLibrary.BreakVector` (`self.TempPos`)))
  (bind _asplayer_chara_bp (cast `/Game/BP/PlayerCharaBP` (`GameplayStatics.GetPlayerPawn` 0)))
  (set `self.TempPos` (`self.K2_GetActorLocation` _asplayer_chara_bp))
  (`self.K2_SetActorRotation` (`KismetMathLibrary.FindLookAtRotation` (`self.StartPos`) (`KismetMathLibrary.MakeVector` _temppos_x _playerpos_y _playerpos_z)))
  (set `self.flyingTimer` (+ (`self.flyingTimer`) DeltaSeconds))
  (if (>= _temppos_x_2 _returnvalue_x)
    (`self.K2_DestroyActor`)))

(fn `UserConstructionScript`)