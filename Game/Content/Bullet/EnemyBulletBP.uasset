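; Enemy bullet actor that damages whatever lies just ahead of it and expires after a short fixed lifespan.
; Each Tick runs a short Visibility line trace along its forward vector, with the overlap event left empty.
; On a hit it calls ApplyDamage on the hit actor and an emitter spawn at its location.
; It prints player-hit and destroy messages without checking the actor type or destroying itself.
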(event `self.ReceiveBeginPlay`
  (`self.SetLifeSpan` 3.0) ; Destroy after appointed times
)

(event `self.ReceiveTick`
  (params (DeltaSeconds :type "Float (single-precision)"))
  (bind _returnvalue (`self.K2_GetActorLocation`))
  (bind (_outhit _returnvalue_2) (`KismetSystemLibrary.LineTraceSingle` :`Start` _returnvalue :`End` (+ _returnvalue (* (`KismetMathLibrary.GetForwardVector` (`self.K2_GetActorRotation`)) 50.0)) :`TraceChannel` "TraceTypeQuery1" :`TraceColor` (struct :`R` 1.0) :`TraceHitColor` (struct))) ; 線を伸ばして、遮られた位置を判定する
  (if _returnvalue_2
    (`KismetSystemLibrary.PrintString` "HitPlayer")
    (`GameplayStatics.ApplyDamage` (`.HitActor` (`GameplayStatics.BreakHitResult` _outhit)) 0.0 null self)
    (`GameplayStatics.SpawnEmitterAtLocation` null (`self.K2_GetActorLocation`)) ; prevent the effect when hit
    (`KismetSystemLibrary.PrintString` "EnemyBulletGotDestory")))

(fn `UserConstructionScript`)