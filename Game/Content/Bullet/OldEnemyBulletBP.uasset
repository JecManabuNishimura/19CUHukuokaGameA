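; OldEnemyBulletBP is an enemy bullet that reacts to being blocked by the player's guard, apparently an older version.
; The first overlap with an actor tagged "Guard" sets IsGuard, prints a debug message and increments TutorialNum and SuccessCount on the player's PlayerCharaBP.
; Once guarded, Tick pushes the bullet along world +X by a fixed step each frame, without delta-time scaling.
; No unguarded movement is defined in these graphs.
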(event `self.ReceiveActorBeginOverlap`
  (params (OtherActor :type "Actor Object Reference"))
  (if (`self.ActorHasTag` OtherActor "Guard")
    (`/Engine/EditorBlueprintResources/StandardMacros.DoOnce` false
      (:`Completed`
        (set `self.IsGuard` true)
        (bind _asplayer_chara_bp (cast `/Game/BP/PlayerCharaBP` (`GameplayStatics.GetPlayerPawn` 0)))
        (`KismetSystemLibrary.PrintString` "Hello")
        (set `/Game/BP/PlayerCharaBP.TutorialNum` (+ (`/Game/BP/PlayerCharaBP.TutorialNum` _asplayer_chara_bp) 1) _asplayer_chara_bp)
        (set `/Game/BP/PlayerCharaBP.SuccessCount` (+ (`/Game/BP/PlayerCharaBP.SuccessCount` _asplayer_chara_bp) 1) _asplayer_chara_bp)))))

(event `self.ReceiveTick`
  (params (DeltaSeconds :type "Float (single-precision)"))
  (bind (_returnvalue_x _returnvalue_y _returnvalue_z) (`KismetMathLibrary.BreakVector` (`self.K2_GetActorLocation`)))
  (if (`self.IsGuard`)
    (`self.K2_SetActorLocation` (`KismetMathLibrary.MakeVector` (+ _returnvalue_x 300.0) _returnvalue_y _returnvalue_z))))

(fn `UserConstructionScript`)