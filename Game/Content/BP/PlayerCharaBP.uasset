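; Player character Blueprint that adds guard, dash and audio presentation, plus goal-time ranking page controls.
; BeginPlay spawns sound and BGM actors attached to the capsule.
; Tick polls the player pawn's state, spawning or destroying a GuardBP actor as guarding changes and toggling post-process blend weight while dashing.
; After the goal, Left/Right key flags change the clamped page number and reload UI_RankingList widgets, clearing the flags afterwards.
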(event `self.ReceiveActorBeginOverlap`
  (params (OtherActor :type "Actor Object Reference")))

(event `self.ReceiveBeginPlay`
  (bind _returnvalue (`|SpawnActorFromClass` "/Game/BP/SoundsBP/PlayerSounds.PlayerSounds_C" (`self.SoundsPos`) "AdjustIfPossibleButAlwaysSpawn" "OverrideRootScale" null null))
  (`self.K2_AttachToComponent` _returnvalue (`self.CapsuleComponent`) "None" "KeepRelative" "KeepRelative" "KeepRelative" true)
  (bind _returnvalue_2 (`|SpawnActorFromClass` "/Game/BP/SoundsBP/GameBGM.GameBGM_C" (`self.SoundsPos`) "AdjustIfPossibleButAlwaysSpawn" "OverrideRootScale" null null))
  (`self.K2_AttachToComponent` _returnvalue_2 (`self.CapsuleComponent`) "None" "KeepRelative" "KeepRelative" "KeepRelative" true))

(event `self.ReceiveTick`
  (params (DeltaSeconds :type "Float (single-precision)"))
  (bind _postprocess (`self.PostProcess`))
  (`|ExecutionSequence`
    (:`then_0`
      ;[1 1 1] スコアタグの生成
      (bind _asplayer_chara_bp (cast `/Game/BP/PlayerCharaBP` (`GameplayStatics.GetPlayerPawn` 0)))
      (if (`PlayerChara.isGuarding` _asplayer_chara_bp)
        (if (`self.IsGenerateGuard_0`)
          (if (`PlayerChara.isGoal` _asplayer_chara_bp) :!label _label
            (if (`self.NextPage`)
              (bind _nowpage (`PlayerChara.nowPage` _asplayer_chara_bp))
              (if (< _nowpage (`PlayerChara.maxPage` _asplayer_chara_bp))
                (set `PlayerChara.nowPage` (+ _nowpage 1) _asplayer_chara_bp)
                (bind _foundwidgets (`WidgetBlueprintLibrary.GetAllWidgetsOfClass` "/Game/UI/UI_RankingList.UI_RankingList_C"))
                (for _array_element _foundwidgets
                  (set `self.RankList` _array_element)
                  (`/Game/UI/UI_RankingList.LoadData` (`self.RankList`))
                  (set `self.NextPage` false)
                  (set `self.PrePage` false)))
              (elif (`self.PrePage`)
                (if (> _nowpage 1)
                  (set `PlayerChara.nowPage` (- _nowpage 1) _asplayer_chara_bp)
                  (bind _foundwidgets_2 (`WidgetBlueprintLibrary.GetAllWidgetsOfClass` "/Game/UI/UI_RankingList.UI_RankingList_C"))
                  (for _array_element_2 _foundwidgets_2
                    (set `self.RankList` _array_element_2)
                    (`/Game/UI/UI_RankingList.LoadData` (`self.RankList`))
                    (set `self.PrePage` false)
                    (set `self.NextPage` false))))))
          (else
            (bind _returnvalue (`|SpawnActorFromClass` "/Game/BP/GuardBP.GuardBP_C" (`self.GuardPos`) "AdjustIfPossibleButAlwaysSpawn" "OverrideRootScale" null null))
            (set `self.IsGenerateGuard_0` true)))
        (elif (`self.IsGenerateGuard_0`)
          (`self.K2_DestroyActor` _returnvalue)
          (set `self.IsGenerateGuard_0` false)
          (else
            (goto _label)))))
    (:`then_1`
      ;[1 1 1] ダッシュの生成（PostProcess）
      (bind _asplayer_chara (cast `PlayerChara` (`GameplayStatics.GetPlayerPawn` 0)))
      (if (`PlayerChara.isDashing` _asplayer_chara)
        (set `PostProcessComponent.BlendWeight` 1.0 _postprocess)
        (else
          (set `PostProcessComponent.BlendWeight` 0.0 _postprocess))))))

(event `Key|Right`
  (params (Key :type "Key Structure"))
  (:`Pressed`
    (set `self.NextPage` true))
  (:`Released`
    (set `self.NextPage` false)))

(event `Key|Left`
  (params (Key :type "Key Structure"))
  (:`Pressed`
    (set `self.PrePage` true))
  (:`Released`
    (set `self.PrePage` false)))

(fn `UserConstructionScript`)