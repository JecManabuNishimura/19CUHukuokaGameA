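; StartBP is a stage select actor that shows the start icon and handles the door-opening transition into the Loading level.
; Each Tick reads flags on the StageSelectCameraBP pawn, holding both doors in idle while a timer runs when UI display is allowed.
; The timer then spawns StartIconBP, attaches it to the camera and clears that flag.
; Afterwards, Enter with start attached plays the door move animations and loads the level after a delay.
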(event `self.ReceiveTick`
  (params (DeltaSeconds :type "Float (single-precision)"))
  (bind _asstage_select_camera_bp (cast `/Game/BP/StageSelect/StageSelectCameraBP` (`GameplayStatics.GetPlayerPawn` 0)))
  (if (`StageSelectCamera.canDisplayUI` _asstage_select_camera_bp)
    (`SkeletalMeshComponent.PlayAnimation` (`self.LeftDoor`) "/Game/Title/Door/Door_Animation/Door_Idle/Door1_1_Idle.Door1_1_Idle" false)
    (`SkeletalMeshComponent.PlayAnimation` (`self.RightDoor`) "/Game/Title/Door/Door_Animation/Door_Idle/Door1_2_Idle.Door1_2_Idle" false)
    (bind _output_get (set `self.CountTime` (+ (`self.CountTime`) (* (`self.TimeRate`) DeltaSeconds))))
    (if (>= _output_get 1.0)
      (set `self.CountTime` 0.0)
      (bind _returnvalue (`|SpawnActorFromClass` "/Game/BP/StageSelect/StartIconBP.StartIconBP_C" (`KismetMathLibrary.MakeTransform` (300.0 0.0 0.0) (struct :`Yaw` 180.0) (0.3 0.3 0.3)) "AdjustIfPossibleButAlwaysSpawn" "OverrideRootScale" null null))
      (bind _asstage_select_camera_bp_2 (cast `/Game/BP/StageSelect/StageSelectCameraBP` (`GameplayStatics.GetPlayerPawn` 0)))
      (`self.K2_AttachToComponent` _returnvalue (`Actor.RootComponent` _asstage_select_camera_bp_2) "None" "KeepRelative" "KeepRelative" "KeepRelative" true)
      (set `StageSelectCamera.canDisplayUI` false _asstage_select_camera_bp_2))
    (elif (and (`StageSelectCamera.isEnterButtonPressed` _asstage_select_camera_bp) (`StageSelectCamera.isStartAttached` _asstage_select_camera_bp))
      (`SkeletalMeshComponent.PlayAnimation` (`self.LeftDoor`) "/Game/Title/Door/Door_Animation/Door_Move/Door1_1_Move.Door1_1_Move" false)
      (`SkeletalMeshComponent.PlayAnimation` (`self.RightDoor`) "/Game/Title/Door/Door_Animation/Door_Move/Door1_2_Move.Door1_2_Move" false)
      (`KismetSystemLibrary.Delay` 3.0)
      (`GameplayStatics.OpenLevel` "Loading"))))

(fn `UserConstructionScript`)