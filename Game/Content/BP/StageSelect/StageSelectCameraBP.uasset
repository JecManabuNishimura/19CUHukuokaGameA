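; Stage select camera Blueprint that sets floor tracking origin and handles Select and Decide sound effects for menu input.
; Left/Right and Enter/Backspace set flags that Tick reads while the stage select or start screen is attached.
; Select stays rewound and paused until a direction is held; Decide plays once per press via a DoOnce reset on release.
; StageSelectBP respawn logic is left unconnected and never runs.
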(event `self.ReceiveBeginPlay`
  (`HeadMountedDisplayFunctionLibrary.SetTrackingOrigin` "Floor")
  (`AudioComponent.SetPaused` (`self.Decide`) true)
  (`AudioComponent.SetPaused` (`self.Select`) true))

(event `self.ReceiveTick`
  (params (DeltaSeconds :type "Float (single-precision)"))
  (bind _select (`self.Select`))
  (bind _decide (`self.Decide`))
  (if (or (`self.isStageSelectAttached`) (`self.isStartAttached`))
    ;[1 1 1] SE
    (if (`self.IsSelecting`)
      (if (`self.isStageSelectAttached`)
        (`AudioComponent.SetPaused` (`self.Select`) false))
      (else
        (`AudioComponent.Play` _select 0.0)
        (`AudioComponent.SetPaused` _select true)
        (if (and (`self.IsDecided`) (or (`self.isEnterButtonPressed`) (`self.isCancelButtonPressed`)))
          (`/Engine/EditorBlueprintResources/StandardMacros.DoOnce` false :!label _label
            (:`Completed`
              (`AudioComponent.SetPaused` _decide false)
              (`AudioComponent.Play` _decide 0.0)
              (`KismetSystemLibrary.Delay` 1.2))))))))

(event `Key|Right`
  (params (Key :type "Key Structure"))
  (:`Pressed`
    (set `self.IsSelecting` true :!label _label_2))
  (:`Released`
    (set `self.IsSelecting` false :!label _label_3)))

(event `Key|Left`
  (params (Key :type "Key Structure"))
  (:`Pressed`
    (goto _label_2))
  (:`Released`
    (goto _label_3)))

(event `Key|Enter`
  (params (Key :type "Key Structure"))
  (:`Pressed`
    (set `self.IsDecided` true :!label _label_4))
  (:`Released`
    (set `self.IsDecided` false :!label _label_5)
    (goto _label :!via `Reset`)))

(event `Key|BackSpace`
  (params (Key :type "Key Structure"))
  (:`Pressed`
    (goto _label_4))
  (:`Released`
    (goto _label_5)))

(fn `UserConstructionScript`)