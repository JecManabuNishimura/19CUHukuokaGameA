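; Stage select actor that stores the chosen stage in the game instance and loads the Game level on confirmation.
; Left and Right keys set a selecting flag; while held, Tick unpauses the Select audio and writes CurrentStage to BP_MyInstance's StageNum.
; When not selecting, Tick restarts and pauses Select, and an Enter press triggers a one-shot Decide playback followed by a short delay before the level opens.
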(event `self.ReceiveBeginPlay`
  (`AudioComponent.SetPaused` (`self.Decide`) true))

(event `self.ReceiveTick`
  (params (DeltaSeconds :type "Float (single-precision)"))
  (bind _select (`self.Select`))
  (bind _decide (`self.Decide`))
  (if (`self.IsSelecting`)
    (`AudioComponent.SetPaused` (`self.Select`) false)
    (bind _asbp_my_instance (cast `/Game/BP/PlayerData/BP_MyInstance` (`GameplayStatics.GetGameInstance`)))
    (set `/Game/BP/PlayerData/BP_MyInstance.StageNum` (`self.currentStage`) _asbp_my_instance)
    (else
      (`AudioComponent.Play` _select 0.0)
      (`AudioComponent.SetPaused` _select true)
      (if (`self.IsDecided`)
        (`/Engine/EditorBlueprintResources/StandardMacros.DoOnce` false
          (:`Completed`
            (`AudioComponent.SetPaused` _decide false)
            (`AudioComponent.Play` _decide 0.0)
            (`KismetSystemLibrary.Delay` 1.2)
            (`GameplayStatics.OpenLevel` "Game")))))))

(event `Key|Right`
  (params (Key :type "Key Structure"))
  (:`Pressed`
    (set `self.IsSelecting` true :!label _label))
  (:`Released`
    (set `self.IsSelecting` false :!label _label_2)))

(event `Key|Left`
  (params (Key :type "Key Structure"))
  (:`Pressed`
    (goto _label))
  (:`Released`
    (goto _label_2)))

(event `Key|Enter`
  (params (Key :type "Key Structure"))
  (:`Pressed`
    (set `self.IsDecided` true))
  (:`Released`
    (set `self.IsDecided` false)))

(fn `UserConstructionScript`)