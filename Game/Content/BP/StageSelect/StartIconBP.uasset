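; StartIconBP is the start icon actor in stage select, which reacts to the confirm and cancel states of the StageSelectCameraBP player pawn.
; It pauses its Decide component on BeginPlay, then polls the pawn's button flags every Tick.
; Enter opens the Loading level after a one-second delay.
; Cancel clears the pawn's IsStartAttached flag and destroys the icon.
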(event `self.ReceiveBeginPlay`
  (`AudioComponent.SetPaused` (`self.Decide`) true))

(event `self.ReceiveTick`
  (params (DeltaSeconds :type "Float (single-precision)"))
  (bind _asstage_select_camera_bp (cast `/Game/BP/StageSelect/StageSelectCameraBP` (`GameplayStatics.GetPlayerPawn` 0)))
  (if (`StageSelectCamera.isEnterButtonPressed` _asstage_select_camera_bp)
    (`KismetSystemLibrary.Delay` 1.0)
    (`GameplayStatics.OpenLevel` "Loading")
    (elif (`StageSelectCamera.isCancelButtonPressed` _asstage_select_camera_bp)
      (set `StageSelectCamera.isStartAttached` false _asstage_select_camera_bp)
      (`self.K2_DestroyActor`))))

(fn `UserConstructionScript`)