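; Name-input Blueprint, judging by its name, that plays select, decide and cancel audio feedback and hands off to the Loading level.
; Up/Down, Enter and SpaceBar set flags that Tick polls to unpause each sound, otherwise restarting and pausing it, with delays clearing decide and cancel.
; When ConfirmIndex, not changed here, reaches its final value, a DoOnce plays the decide sound and opens Loading after a delay.
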(event `self.ReceiveBeginPlay`)

(event `self.ReceiveTick`
  (params (DeltaSeconds :type "Float (single-precision)"))
  (bind _decide (`self.Decide`))
  (bind _cancel (`self.Cancel`))
  (bind _select (`self.Select`))
  (bind _decide_2 (`self.Decide`))
  (if (`self.IsSelecting`)
    (`AudioComponent.SetPaused` (`self.Select`) false)
    (else
      (`AudioComponent.Play` _select 0.0)
      (`AudioComponent.SetPaused` _select true)
      (if (== (`self.confirmIndex`) 5)
        (`/Engine/EditorBlueprintResources/StandardMacros.DoOnce` false
          (:`Completed`
            (`AudioComponent.SetPaused` _decide_2 false)
            (`AudioComponent.Play` _decide_2 0.0)
            (`KismetSystemLibrary.Delay` 1.2)
            (`GameplayStatics.OpenLevel` "Loading")))
        (elif (`self.IsDecided`)
          (`AudioComponent.SetPaused` (`self.Decide`) false)
          (`KismetSystemLibrary.Delay` 0.7)
          (set `self.IsDecided` false)
          (else
            (`AudioComponent.Play` _decide 0.0)
            (`AudioComponent.SetPaused` _decide true)
            (if (`self.IsCanceled`)
              (`AudioComponent.SetPaused` (`self.Cancel`) false)
              (`KismetSystemLibrary.Delay` 1.0)
              (set `self.IsCanceled` false)
              (else
                (`AudioComponent.Play` _cancel 0.0)
                (`AudioComponent.SetPaused` _cancel true)))))))))

(event `Key|Up`
  (params (Key :type "Key Structure"))
  (:`Pressed`
    (set `self.IsSelecting` true :!label _label))
  (:`Released`
    (set `self.IsSelecting` false :!label _label_2)))

(event `Key|Down`
  (params (Key :type "Key Structure"))
  (:`Pressed`
    (goto _label))
  (:`Released`
    (goto _label_2)))

(event `Key|Enter`
  (params (Key :type "Key Structure"))
  (:`Pressed`
    (set `self.IsDecided` true)))

(event `Key|SpaceBar`
  (params (Key :type "Key Structure"))
  (:`Pressed`
    (set `self.IsCanceled` true)))

(fn `UserConstructionScript`)