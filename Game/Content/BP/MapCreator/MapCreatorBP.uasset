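; MapCreatorBP is an unfinished map builder that reads map layouts from the MapTable data table at BeginPlay.
; It loads rows by sequential numeric name from 1 until a lookup fails, trimming the decimals from a float-to-string conversion.
; Each row's fourteen Line fields become an array fed to a switch with no case logic.
; A SpawnActor node is unconnected, so nothing is spawned yet.
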(event `self.ReceiveBeginPlay`
  (if true
    (set `self.rowIndex` 1)
    (set `self.loadMapData` true)
    (while (`self.loadMapData`)
      (bind _returnvalue (`|GetDataTableRow` (`self.MapTable`) (`KismetStringLibrary.Conv_StringToName` (`KismetStringLibrary.Split` (`KismetStringLibrary.Conv_DoubleToString` (`KismetMathLibrary.Conv_IntToDouble` (`self.rowIndex`))) ".")))
        (:`then`
          (`/Engine/EditorBlueprintResources/StandardMacros.IncrementInt` (`self.rowIndex`)
            (:`  `
              (bind _output_get (set `self.MapStruct` _returnvalue))
              (set `self.strTempArray` (`|MakeArray` (break `/Game/BP/MapCreator/MapStruct` _output_get) (`.Line_2_12_738A2F864A6B1FF22137D784F45D1435` (break `/Game/BP/MapCreator/MapStruct` _output_get)) (`.Line_3_13_C4F3A55D4530BBC093433995CDD73008` (break `/Game/BP/MapCreator/MapStruct` _output_get)) (`.Line_4_14_3F07A5684558F3B1CADAE6A8CE882E25` (break `/Game/BP/MapCreator/MapStruct` _output_get)) (`.Line_5_15_F1B2A45F4A6690D52CC405866CE67BEB` (break `/Game/BP/MapCreator/MapStruct` _output_get)) (`.Line_6_23_0C2F00F0479059E0CD251091A37ED0F1` (break `/Game/BP/MapCreator/MapStruct` _output_get)) (`.Line_7_24_BD410A024D17D780B179AD96455D379B` (break `/Game/BP/MapCreator/MapStruct` _output_get)) (`.Line_8_25_540137734F260A1C00D92EAD28F48C0B` (break `/Game/BP/MapCreator/MapStruct` _output_get)) (`.Line_9_26_134E83144515B3C9D54BA0B6ABC27E44` (break `/Game/BP/MapCreator/MapStruct` _output_get)) (`.Line_10_27_EEEE9E7C42F43FA169104090FCA7FC0F` (break `/Game/BP/MapCreator/MapStruct` _output_get)) (`.Line_11_28_E8D0C35C4483B3118A9592932A18D655` (break `/Game/BP/MapCreator/MapStruct` _output_get)) (`.Line_12_30_D6AF47CA4A353B78CC4AED8F4B3A1BA4` (break `/Game/BP/MapCreator/MapStruct` _output_get)) (`.Line_13_32_DE37CFA840FE65D069C82898FB02941A` (break `/Game/BP/MapCreator/MapStruct` _output_get)) (`.Line_14_34_0105AD8146CD3DBA6E1A0BAFFD8A3155` (break `/Game/BP/MapCreator/MapStruct` _output_get))))
              (for _index (range (+ (`KismetArrayLibrary.Array_Length` (`self.strTempArray`)) 1))
                (switch `string` (`|GetArrayItem` (`self.strTempArray`) _index))))))
        (:`RowNotFound`
          (set `self.loadMapData` false))))))

(fn `UserConstructionScript`)