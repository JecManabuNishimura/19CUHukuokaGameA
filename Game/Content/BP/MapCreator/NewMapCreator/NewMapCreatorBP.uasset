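; Map creator Blueprint that spawns level actors on a row and column grid from map creation data.
; MapCreateBP places Single entries individually and spawns horizontal fences as one scaled actor centred on the linked span, using index counters to avoid duplicates.
; GetLinkIndexBP resolves fence links but compares only the first array element.
; BeginPlay is empty and the setup chain calling MapCreateBP is disconnected, so the file never triggers generation itself.
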(event `self.ReceiveBeginPlay`)

(fn `GetLinkIndexBP`
  (params (_linkIndex :type Integer) (_array :type "Array of ContinuousData Structure"))
  (returns (index :type Integer))
  (locals (result :type Integer))
  (bind _output_linkindex (break `ContinuousData` (`|GetArrayItem` _array)))
  (set `local.result` -1)
  (for _index (range (`KismetArrayLibrary.Array_Length` _array))
    (if (== _linkIndex _output_linkindex)
      (set `local.result` _index)
      (break)))
  (return (`local.result`)))

(fn `LocationX`
  (params (rowIndex :type Integer))
  (returns (locationX :type "Float (double-precision)"))
  (return (* rowIndex (`self.m_XAxis_Offset`))))

(fn `LocationY`
  (params (_columnIndex :type Integer) (_strArrayLength :type Integer))
  (returns (locationY :type "Float (double-precision)"))
  (bind _result (`/Engine/EditorBlueprintResources/StandardMacros.DecrementInt` _strArrayLength)
    (:`  `
      (return (- (`KismetMathLibrary.Conv_IntToDouble` _columnIndex) (/ (`KismetMathLibrary.Conv_IntToDouble` _result) 2.0))))))

(fn `Map Create BP`
  (locals (nowCreateData :type "CreateData Structure"))
  (bind _nowcreatedata (`local.nowCreateData`))
  (bind (_generateactorstruct _rowindex _columnindex) (break `CreateData` _nowcreatedata))
  (bind (_generateactorstruct_2 _rowindex_2 _columnindex_2 _generatestring _generatepattern _isfence _fencestart _vertlinknum) (break `CreateData` _nowcreatedata))
  (bind (_output_linkindex _output_startindex _output_endindex) (break `ContinuousData` (`|GetArrayItem` (`self.m_FenceData`) (`self.fenceDataIndex`))))
  (bind (_output_linkindex_2 _output_startindex_2 _output_endindex_2 _output_scale) (break `ContinuousData` (`|GetArrayItem` (`self.m_FenceData`) (`self.fenceDataIndex`))))
  (set `self.fenceDataIndex` 0)
  (set `self.fenceIndex` 0)
  (for _array_element (`self.m_MapActorCreateData`)
    (bind _output_get (set `local.nowCreateData` _array_element))
    (switch `EMapPlacementPattern` (`.generatePattern` (break `CreateData` _output_get))
      (:`Single`
        (bind _locationx (`self.LocationX` _rowindex))
        (bind _locationy (`self.LocationY` _columnindex (`self.m_StrMapLength`)))
        (`self.SpawnActor` _generateactorstruct _locationx _locationy))
      (:`Fence`
        (bind _index (`self.GetLinkIndexBP` _vertlinknum (`self.m_FenceData`)))
        (bind _output_get_2 (set `self.fenceDataIndex` _index))
        (if (== _output_get_2 (`self.fenceIndex`))
          (set `self.actorTemp` _generateactorstruct_2)
          (set `self.actorTemp` (make `MapActorStructCpp` null 0.0 (struct) _output_scale))
          (bind _locationx_2 (`self.LocationX` (`.rowIndex` (break `CreateData` _nowcreatedata))))
          (bind _locationy_2 (`self.LocationY` (/ (+ _output_startindex _output_endindex) 2) (`self.m_StrMapLength`)))
          (`self.SpawnActor` (`self.actorTemp`) _locationx_2 _locationy_2)
          (`/Engine/EditorBlueprintResources/StandardMacros.IncrementInt` (`self.fenceIndex`)))))))

(fn `SpawnActor`
  (params (_spawnActor :type "MapActorStructCpp Structure") (_locationX :type "Float (double-precision)") (_locationY :type "Float (double-precision)"))
  (returns (spawnedActor :type "Actor Object Reference"))
  (bind _returnvalue (`|SpawnActorFromClass` _spawnActor_actor (`KismetMathLibrary.MakeTransform` (`KismetMathLibrary.MakeVector` _locationX _locationY _spawnActor_location_Z) _spawnActor_rotation _spawnActor_scale) "Undefined" "OverrideRootScale" null null))
  (return _returnvalue))

(fn `UserConstructionScript`)