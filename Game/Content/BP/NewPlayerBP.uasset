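; Player Blueprint that keeps a board mesh under the character's animated feet and spawns a landing effect.
; BeginPlay records both foot bones' rest heights in component space.
; Each tick, the board's height follows the average foot offset and its pitch follows an Atan2 of the feet's Y-Z difference.
; Two other computed angles and a cosine-based rotation graph go unused.
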(event `self.ReceiveBeginPlay`
  (set `self.LeftFootBoneOriginLocationZ` (.z (.location (`SceneComponent.GetSocketTransform` (`self.m_PlayerMesh`) (`self.LeftFootBoneName`) "RTS_Component"))))
  (set `self.RightFootBoneOriginLocationZ` (.z (.location (`SceneComponent.GetSocketTransform` (`self.m_PlayerMesh`) (`self.RightFootBoneName`) "RTS_Component"))))
  (set `self.OriginRot` (`SceneComponent.RelativeRotation` (`self.m_PlayerMesh`))))

(event `self.ReceiveTick`
  (params (DeltaSeconds :type "Float (single-precision)"))
  (bind _returnvalue (`self.GetTransform`))
  (`|ExecutionSequence`
    (:`then_0`
      (`self.SetBoardLocationAndRotation`))
    (:`then_1`
      (if (`self.GetLanding`)
        (`NiagaraFunctionLibrary.SpawnSystemAtLocation` "/Game/NewCyfer/Assets/Effect/Landing/Effect/Smoke/Landing.Landing" (`KismetMathLibrary.MakeVector` (.x (.location _returnvalue)) (.y (.location _returnvalue)) (.z (.location _returnvalue))))))))

(fn `SetBoardLocationAndRotation`
  (locals (bunbo :type "Float (double-precision)") (bunshi :type "Float (double-precision)") (LeftFootBoneLocation :type "Vector Structure") (RightFootBoneLocation :type "Vector Structure") (Vector2DArray :type "Array of Vector2D Structure") (RotationTemp :type "Array of Float (double-precision)"))
  (bind (_leftfootbonelocation_x _leftfootbonelocation_y _leftfootbonelocation_z) (`KismetMathLibrary.BreakVector` (`local.LeftFootBoneLocation`)))
  (bind (_rightfootbonelocation_x _rightfootbonelocation_y _rightfootbonelocation_z) (`KismetMathLibrary.BreakVector` (`local.RightFootBoneLocation`)))
  (bind _m_boardmesh (`self.m_BoardMesh`))
  (bind (_leftfootbonelocation_x_2 _leftfootbonelocation_y_2 _leftfootbonelocation_z_2) (`KismetMathLibrary.BreakVector` (`local.LeftFootBoneLocation`)))
  (bind (_rightfootbonelocation_x_2 _rightfootbonelocation_y_2 _rightfootbonelocation_z_2) (`KismetMathLibrary.BreakVector` (`local.RightFootBoneLocation`)))
  (bind _returnvalue_location (`KismetMathLibrary.BreakTransform` (`SceneComponent.GetSocketTransform` (`self.m_PlayerMesh`) (`self.LeftFootBoneName`) "RTS_Component")))
  (bind _returnvalue_location_2 (`KismetMathLibrary.BreakTransform` (`SceneComponent.GetSocketTransform` (`self.m_PlayerMesh`) (`self.RightFootBoneName`) "RTS_Component")))
  (bind (_relativelocation_x _relativelocation_y) (`KismetMathLibrary.BreakVector` (`SceneComponent.RelativeLocation` _m_boardmesh)))
  (`|ExecutionSequence`
    (:`then_0`
      (bind _output_get (set `local.LeftFootBoneLocation` _returnvalue_location))
      (bind _output_get_2 (set `local.RightFootBoneLocation` _returnvalue_location_2))
      (`SceneComponent.K2_SetRelativeLocation` _m_boardmesh (`KismetMathLibrary.MakeVector` _relativelocation_x _relativelocation_y (- (/ (+ _leftfootbonelocation_z _rightfootbonelocation_z) 2.0) (/ (+ (`self.LeftFootBoneOriginLocationZ`) (`self.RightFootBoneOriginLocationZ`)) 2.0))) false false))
    (:`then_1`
      (set `local.Vector2DArray` (`|MakeArray` (`KismetMathLibrary.MakeVector2D` _leftfootbonelocation_y_2 _leftfootbonelocation_z_2) (`KismetMathLibrary.MakeVector2D` _rightfootbonelocation_y_2 _rightfootbonelocation_z_2) (`KismetMathLibrary.MakeVector2D` _leftfootbonelocation_x_2 _leftfootbonelocation_z_2) (`KismetMathLibrary.MakeVector2D` _rightfootbonelocation_x_2 _rightfootbonelocation_z_2) (`KismetMathLibrary.MakeVector2D` _leftfootbonelocation_x_2 _leftfootbonelocation_y_2) (`KismetMathLibrary.MakeVector2D` _rightfootbonelocation_x_2 _rightfootbonelocation_y_2) :!type "Vector2D Structure"))
      (`KismetArrayLibrary.Array_Clear` (`local.RotationTemp`))
      (for _index (range 3)
        (bind _returnvalue (* _index 2))
        (bind (_output_x _output_y) (`KismetMathLibrary.BreakVector2D` (`|GetArrayItem` (`local.Vector2DArray`) (+ _returnvalue 1))))
        (bind (_output_x_2 _output_y_2) (`KismetMathLibrary.BreakVector2D` (`|GetArrayItem` (`local.Vector2DArray`) _returnvalue)))
        (`KismetArrayLibrary.Array_Add` (`local.RotationTemp`) (`KismetMathLibrary.DegAtan2` (- _output_y _output_y_2) (- _output_x _output_x_2))))
      (`SceneComponent.K2_SetRelativeRotation` (`self.m_BoardMesh`) (`KismetMathLibrary.MakeRotator` 0.0 (`|GetArrayItem` (`local.RotationTemp`)) 90.0) false false))))

(fn `UserConstructionScript`)