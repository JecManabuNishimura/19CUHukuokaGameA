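; Title screen actor that plays the title music, waits for any key, and moves the game on to the Loading level.
; BeginPlay holds the Title component paused; a key press unpauses it and sets IsPressedInTitle on ZonJyaton_GameMode.
; Tick polls the game mode's AnimationFinishedInTitle flag, which is set outside this Blueprint, and opens Loading after a short delay once it is true.
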(event `self.ReceiveBeginPlay`
  (`AudioComponent.SetPaused` (`self.Title`) true)
  (`AudioComponent.Play` (`self.TitleBGM`) 0.0))

(event `self.ReceiveTick`
  (params (DeltaSeconds :type "Float (single-precision)"))
  (bind _aszon_jyaton_game_mode (cast `/Game/BP/ZonJyaton_GameMode` (`GameplayStatics.GetGameMode`)))
  (if (`/Game/BP/ZonJyaton_GameMode.AnimationFinishedInTitle` _aszon_jyaton_game_mode)
    (`KismetSystemLibrary.Delay` 0.4)
    (`GameplayStatics.OpenLevel` "Loading")))

(event `Key|AnyKey`
  (params (Key :type "Key Structure"))
  (:`Pressed`
    (bind _aszon_jyaton_game_mode (cast `/Game/BP/ZonJyaton_GameMode` (`GameplayStatics.GetGameMode`)))
    (set `/Game/BP/ZonJyaton_GameMode.isPressedInTitle` true _aszon_jyaton_game_mode)
    (`AudioComponent.SetPaused` (`self.Title`) false)))

(fn `UserConstructionScript`)