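; Player-following camera actor that also handles dash/guard effects and spawns HUD, goal and death UI for flat-screen and VR play.
; Tick tilts pitch on SightChange, trails the player from above, and shifts FOV and post-process while dashing.
; BeginPlay attaches effect actors and VR-only 3D HUD panels to the camera.
; Falling below a Z threshold flags death, sinks the camera and triggers glitch and death UI; reaching the goal shows results.
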(event `self.ReceiveTick`
  (params (DeltaSeconds :type "Float (single-precision)"))
  (bind (_returnvalue_x _returnvalue_y) (`KismetMathLibrary.BreakVector` (`self.K2_GetActorLocation`)))
  (bind (_returnvalue_x_2 _returnvalue_y_2 _returnvalue_z) (`KismetMathLibrary.BreakVector` (`self.K2_GetActorLocation`)))
  (bind (_returnvalue_roll _returnvalue_pitch) (`KismetMathLibrary.BreakRotator` (`self.K2_GetActorRotation`)))
  (bind (_returnvalue_roll_2 _returnvalue_pitch_2) (`KismetMathLibrary.BreakRotator` (`self.K2_GetActorRotation`)))
  (bind _dashbp (`self.DashBP`))
  (bind _guardbp (`self.guardBP`))
  (bind _postprocess (`self.PostProcess`))
  (bind _asplayer_chara_bp (cast `/Game/BP/PlayerCharaBP` (`GameplayStatics.GetPlayerPawn` 0)))
  (if (`/Game/BP/PlayerCharaBP.SightChange` _asplayer_chara_bp)
    (if (>= _returnvalue_pitch_2 -20.0)
      (`self.K2_SetActorRotation` (`KismetMathLibrary.MakeRotator` 0.0 (- _returnvalue_pitch_2 1.0))))
    (elif (<= _returnvalue_pitch 0.0)
      (`self.K2_SetActorRotation` (`KismetMathLibrary.MakeRotator` 0.0 (+ _returnvalue_pitch 1.0)))))
  (if (`PlayerChara.isGoal` _asplayer_chara_bp)
    (set `PostProcessComponent.BlendWeight` 0.0 (`self.PostProcess`))
    (`SceneComponent.SetHiddenInGame` (`self.Dash`) false false)
    (`SceneComponent.SetHiddenInGame` (`self.Guard`) false false)
    (bind _asbp_my_instance (cast `/Game/BP/PlayerData/BP_MyInstance` (`GameplayStatics.GetGameInstance`)))
    (if (`/Game/BP/PlayerData/BP_MyInstance.isUsedInVR` _asbp_my_instance)
      (if (`self.GoalCanSpawned`)
        (bind _returnvalue (`|SpawnActorFromClass` "/Game/BP/forVR/VR_UI_Goal.VR_UI_Goal_C" (`KismetMathLibrary.MakeTransform` (+ (`self.K2_GetActorLocation`) (1000.0 0.0 200.0)) (struct :`Yaw` 180.0)) "AlwaysSpawn" "OverrideRootScale" null null))
        (set `self.GoalCanSpawned` false)
        (else
          (bind _asplayer_chara_bp_2 (cast `/Game/BP/PlayerCharaBP` (`GameplayStatics.GetPlayerPawn` 0)))
          (if (`PlayerChara.haveShowedRanking` _asplayer_chara_bp_2)
            (`self.K2_DestroyActor` _returnvalue)
            (if (`self.RankCanSpawned`)
              (`|SpawnActorFromClass` "/Game/BP/forVR/VR_UI_RankingList.VR_UI_RankingList_C" (`KismetMathLibrary.MakeTransform` (+ (`self.K2_GetActorLocation`) (1500.0 0.0 200.0)) (struct :`Yaw` 180.0)) "AlwaysSpawn" "OverrideRootScale" null null)
              (set `self.RankCanSpawned` false)))))
      (else
        (`/Engine/EditorBlueprintResources/StandardMacros.DoOnce` false
          (:`Completed`
            (bind _returnvalue_2 (`|CreateWidget` "/Game/UI/UI_Goal.UI_Goal_C"))
            (`UserWidget.AddToViewport` _returnvalue_2 0)))))
    (else
      (`|ExecutionSequence`
        (:`then_0`
          (bind _asplayer_chara_bp_3 (cast `/Game/BP/PlayerCharaBP` (`GameplayStatics.GetPlayerPawn` 0)))
          (if (< _returnvalue_z -1000.0)
            (set `PlayerChara.isDead` true _asplayer_chara_bp_3)
            (set `self.DeadPosZ` (- (`self.DeadPosZ`) 20.0))
            (`self.K2_SetActorLocation` (`KismetMathLibrary.MakeVector` _returnvalue_x _returnvalue_y (`self.DeadPosZ`)))
            (`/Engine/EditorBlueprintResources/StandardMacros.DoOnce` false
              (:`Completed`
                (`/Engine/EditorBlueprintResources/StandardMacros.DoOnce` false
                  (:`Completed`
                    (`NiagaraFunctionLibrary.SpawnSystemAttached` "/Game/Effect/GameOverGlitch/Glitch_Ns.Glitch_NS" (`self.DefaultSceneRoot`) "None" (0.0 0.0 0.0) (struct) "KeepRelativeOffset")
                    (`KismetSystemLibrary.Delay` (`self.BlackStartDelay`))
                    (bind _returnvalue_3 (`|CreateWidget` "/Game/UI/PlayerOpa.PlayerOpa_C"))
                    (`UserWidget.AddToViewport` _returnvalue_3 -1)
                    (`KismetSystemLibrary.Delay` 0.5)
                    (bind _returnvalue_4 (`|CreateWidget` "/Game/UI/UI_DeadPlaySelect.UI_DeadPlaySelect_C"))
                    (`UserWidget.AddToViewport` _returnvalue_4 0)
                    (bind _asplayer_chara_bp_4 (cast `/Game/BP/PlayerCharaBP` (`GameplayStatics.GetPlayerPawn` 0)))
                    (set `PlayerChara.haveShowedDeadUI` true _asplayer_chara_bp_4)))))
            (elif (`PlayerChara.isDashLine` _asplayer_chara_bp_3)
              (bind (_returnvalue_x_3 _returnvalue_y_3 _returnvalue_z_2) (`KismetMathLibrary.BreakVector` (`self.K2_GetActorLocation` _asplayer_chara_bp_3)))
              (`self.K2_SetActorLocation` (`KismetMathLibrary.MakeVector` _returnvalue_x_3 _returnvalue_y_3 (+ _returnvalue_z_2 500.0)) :!label _label)
              (if (<= (`self.DownFieldSpeed`) 5.0)
                (bind _output_get (set `self.DownFieldSpeed` (+ (`self.DownFieldSpeed`) 0.4))))
              (if (< (`self.DownField`) 110.0)
                (bind _output_get_2 (set `self.DownField` (+ _output_get (`self.DownField`)))))
              (`CameraComponent.SetFieldOfView` (`self.Camera`) _output_get_2)
              (set `self.UpField` 110.0)
              (elif (`PlayerChara.isDashing` _asplayer_chara_bp_3)
                (goto _label)
                (else
                  (bind (_returnvalue_x_4 _returnvalue_y_4 _returnvalue_z_3) (`KismetMathLibrary.BreakVector` (`self.K2_GetActorLocation` _asplayer_chara_bp_3)))
                  (`self.K2_SetActorLocation` (`KismetMathLibrary.MakeVector` _returnvalue_x_4 _returnvalue_y_4 (+ _returnvalue_z_3 500.0)))
                  (if (> (`self.UpField`) 90.0)
                    (bind _output_get_3 (set `self.UpField` (+ (`self.UpField`) -0.1))))
                  (`CameraComponent.SetFieldOfView` (`self.Camera`) _output_get_3)
                  (set `self.DownField` 90.0)
                  (set `self.DownFieldSpeed` 0.0))))))
        (:`then_1`
          ;[1 1 1] Dashの生成(方法二)
          (bind _asplayer_chara_bp_5 (cast `/Game/BP/PlayerCharaBP` (`GameplayStatics.GetPlayerPawn` 0)))
          (`self.K2_SetActorLocation` _dashbp (`SceneComponent.K2_GetComponentLocation` (`self.Camera`)) false false)
          (`self.SetActorHiddenInGame` _dashbp (not (`PlayerChara.isDashing` _asplayer_chara_bp_5))))
        (:`then_2`
          ;[1 1 1] Guardの生成
          (bind _asplayer_chara_bp_6 (cast `/Game/BP/PlayerCharaBP` (`GameplayStatics.GetPlayerPawn` 0)))
          (`self.K2_SetActorLocation` _guardbp (`SceneComponent.K2_GetComponentLocation` (`self.Camera`)) false false)
          (`self.SetActorHiddenInGame` _guardbp (not (`PlayerChara.isGuarding` _asplayer_chara_bp_6))))
        (:`then_3`
          (bind _asbp_my_instance_2 (cast `/Game/BP/PlayerData/BP_MyInstance` (`GameplayStatics.GetGameInstance`)))
          (if (`/Game/BP/PlayerData/BP_MyInstance.isUsedInVR` _asbp_my_instance_2)
            ;[1 1 1] 死亡UIの生成
            (if (`PlayerChara.isDead` _asplayer_chara_bp)
              (`/Engine/EditorBlueprintResources/StandardMacros.DoOnce` false
                (:`Completed`
                  (`|SpawnActorFromClass` "/Game/BP/forVR/VR_UI_DeadPlaySelect.VR_UI_DeadPlaySelect_C" (`KismetMathLibrary.MakeTransform` (+ (`self.K2_GetActorLocation`) (1500.0 0.0 0.0)) (struct :`Yaw` 180.0)) "AlwaysSpawn" "OverrideRootScale" null null))))))
        (:`then_4`
          ;[1 1 1] ダッシュの生成（PostProcess）
          (bind _asplayer_chara (cast `PlayerChara` (`GameplayStatics.GetPlayerPawn` 0)))
          (if (`PlayerChara.isDashLine` _asplayer_chara)
            (set `PostProcessComponent.BlendWeight` 0.4 _postprocess :!label _label_2)
            (elif (`PlayerChara.isDashing` _asplayer_chara)
              (goto _label_2)
              (else
                (set `PostProcessComponent.BlendWeight` 0.0 _postprocess)))))))))

(event `self.ReceiveBeginPlay`
  ;[1 1 1] 各3DUIの初期配置
  (bind _returnvalue (`|SpawnActorFromClass` "/Game/BP/SphereBP.SphereBP_C" (`KismetMathLibrary.MakeTransform` (`SceneComponent.K2_GetComponentLocation` (`self.DefaultSceneRoot`))) "AdjustIfPossibleButAlwaysSpawn" "OverrideRootScale" null null))
  (bind _output_get (set `self.guardBP` _returnvalue))
  (`self.K2_AttachToComponent` _output_get (`self.Camera`) "None" "KeepRelative" "KeepRelative" "KeepRelative" true)
  (bind _returnvalue_2 (`|SpawnActorFromClass` "/Game/BP/DashBP.DashBP_C" (`KismetMathLibrary.MakeTransform` (`SceneComponent.K2_GetComponentLocation` (`self.DefaultSceneRoot`)) (struct :`Pitch` -90.0) (80.0 80.0 80.0)) "AlwaysSpawn" "OverrideRootScale" null null))
  (bind _output_get_2 (set `self.DashBP` _returnvalue_2))
  (`self.K2_AttachToComponent` _output_get_2 (`self.Camera`) "None" "KeepRelative" "KeepRelative" "KeepRelative" true)
  (bind _asbp_my_instance (cast `/Game/BP/PlayerData/BP_MyInstance` (`GameplayStatics.GetGameInstance`)))
  (if (`/Game/BP/PlayerData/BP_MyInstance.isUsedInVR` _asbp_my_instance)
    (bind _returnvalue_3 (`|SpawnActorFromClass` "/Game/BP/forVR/VR_UI_Dash.VR_UI_Dash_C" (`KismetMathLibrary.MakeTransform` (300.0 -100.0 70.0) (struct :`Yaw` 180.0) (0.2 0.2 0.2)) "AlwaysSpawn" "OverrideRootScale" null null))
    (`self.K2_AttachToComponent` _returnvalue_3 (`self.Camera`) "None" "KeepRelative" "KeepRelative" "KeepRelative" true)
    (bind _returnvalue_4 (`|SpawnActorFromClass` "/Game/BP/forVR/VR_UI_Guard.VR_UI_Guard_C" (`KismetMathLibrary.MakeTransform` (300.0 -100.0 70.0) (struct :`Yaw` 180.0) (0.2 0.2 0.2)) "AlwaysSpawn" "OverrideRootScale" null null))
    (`self.K2_AttachToComponent` _returnvalue_4 (`self.Camera`) "None" "KeepRelative" "KeepRelative" "KeepRelative" true)
    (bind _returnvalue_5 (`|SpawnActorFromClass` "/Game/BP/forVR/VR_UI_Shot.VR_UI_Shot_C" (`KismetMathLibrary.MakeTransform` (300.0 -100.0 70.0) (struct :`Yaw` 180.0) (0.2 0.2 0.2)) "AlwaysSpawn" "OverrideRootScale" null null))
    (`self.K2_AttachToComponent` _returnvalue_5 (`self.Camera`) "None" "KeepRelative" "KeepRelative" "KeepRelative" true)
    (bind _returnvalue_6 (`|SpawnActorFromClass` "/Game/BP/forVR/VR_UI_PassTime.VR_UI_PassTime_C" (`KismetMathLibrary.MakeTransform` (300.0 0.0 50.0) (struct :`Yaw` 180.0) (0.3 0.3 0.3)) "AlwaysSpawn" "OverrideRootScale" null null))
    (`self.K2_AttachToComponent` _returnvalue_6 (`self.Camera`) "None" "KeepRelative" "KeepRelative" "KeepRelative" true)
    (bind _returnvalue_7 (`|SpawnActorFromClass` "/Game/BP/forVR/VR_UI_Score.VR_UI_Score_C" (`KismetMathLibrary.MakeTransform` (300.0 -50.0 -30.0) (struct :`Yaw` 180.0) (0.3 0.3 0.3)) "AlwaysSpawn" "OverrideRootScale" null null))
    (`self.K2_AttachToComponent` _returnvalue_7 (`self.Camera`) "None" "KeepRelative" "KeepRelative" "KeepRelative" true)
    (bind _returnvalue_8 (`|SpawnActorFromClass` "/Game/BP/forVR/VR_UI_HP_Condition.VR_UI_HP_Condition_C" (`KismetMathLibrary.MakeTransform` (500.0 0.0 30.0) (struct :`Yaw` 180.0) (0.6 0.6 0.6)) "AlwaysSpawn" "OverrideRootScale" null null))
    (`self.K2_AttachToComponent` _returnvalue_8 (`self.Camera`) "None" "KeepRelative" "KeepRelative" "KeepRelative" true)))

(fn `UserConstructionScript`)