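; Enemy actor Blueprint that fades out and destroys itself once IsDead is set; this graph holds no attack logic despite the asset name.
; Tick accumulates delta time scaled by DeadEffectDuration, which acts as a speed multiplier, to lerp opacity toward zero.
; It creates dynamic instances of both Sphere materials every dead frame to drive their FadeOut parameter.
; The actor is destroyed when the fade reaches zero.
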(event `self.ReceiveTick`
  (params (DeltaSeconds :type "Float (single-precision)"))
  (if (`self.isDead`)
    ;[1 1 1] Material FadeOut(透明度を徐々に0までにする)
    (bind _output_get (set `self.CountTime` (+ (`self.CountTime`) (* DeltaSeconds (`self.DeadEffectDuration`)))))
    (`|ExecutionSequence`
      (:`then_0`
        (bind _returnvalue (`PrimitiveComponent.CreateDynamicMaterialInstance` (`self.Sphere`) 0 "/Game/EnemyFBX/Dash_Enemy/Dash_Enemy.Dash_Enemy" "None"))
        (`MaterialInstanceDynamic.SetScalarParameterValue` _returnvalue "FadeOut" (`KismetMathLibrary.Lerp` 1.0 0.0 _output_get)))
      (:`then_1`
        (bind _returnvalue_2 (`PrimitiveComponent.CreateDynamicMaterialInstance` (`self.Sphere`) 1 "/Game/EnemyFBX/Dash_Enemy/Dash_Enemy2.Dash_Enemy2" "None"))
        (bind _returnvalue_3 (`KismetMathLibrary.Lerp` 1.0 0.0 _output_get))
        (`MaterialInstanceDynamic.SetScalarParameterValue` _returnvalue_2 "FadeOut" _returnvalue_3))
      (:`then_2`
        (if (<= _returnvalue_3 0.0)
          (`self.K2_DestroyActor`))))))

(fn `UserConstructionScript`)