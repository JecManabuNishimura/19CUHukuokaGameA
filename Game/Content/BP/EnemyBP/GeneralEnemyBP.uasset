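; General enemy actor that follows a preset flight pattern and awards score and a kill count to PlayerCharaBP when player bullets deplete its HP.
; Tick drifts it along X until near the player, then moves it by EnemyType: weave, diagonal, side cut, or turning paths.
; Starting Y sets its side, and most patterns self-destroy past side bounds.
; When flagged to ride a DashEnemy, it destroys itself unless IsRidedOn is set.
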(event `self.ReceiveBeginPlay`
  (bind (_returnvalue_x _returnvalue_y) (`KismetMathLibrary.BreakVector` (`self.K2_GetActorLocation`)))
  (if (< _returnvalue_y 0.0)
    (set `self.IsLeft` true)
    (else
      (set `self.IsLeft` false)))
  (if (== (`self.EnemyType`) 4)
    (if (`self.IsLeft`)
      (`self.K2_SetActorRotation` (struct :`Yaw` -45.0))
      (else
        (`self.K2_SetActorRotation` (struct :`Yaw` 45.0))))))

(event `self.ReceiveActorBeginOverlap`
  (params (OtherActor :type "Actor Object Reference"))
  (if (`self.ActorHasTag` OtherActor "PlayerBullet")
    (set `self.HP` (- (`self.HP`) 1))
    (if (<= (`self.HP`) 0)
      (bind _asplayer_chara_bp (cast `/Game/BP/PlayerCharaBP` (`GameplayStatics.GetPlayerPawn` 0)))
      (set `PlayerChara.PlayerScore` (+ (`PlayerChara.PlayerScore` _asplayer_chara_bp) (`self.GeneralEnemyScore`)) _asplayer_chara_bp)
      (set `PlayerChara.CountShootEnemy` (+ (`PlayerChara.CountShootEnemy` _asplayer_chara_bp) 1) _asplayer_chara_bp)
      (`self.K2_DestroyActor`))))

(event `self.ReceiveTick`
  (params (DeltaSeconds :type "Float (single-precision)"))
  (bind (_returnvalue_x _returnvalue_y _returnvalue_z) (`KismetMathLibrary.BreakVector` (`self.K2_GetActorLocation`)))
  (bind (_returnvalue_x_2 _returnvalue_y_2) (`KismetMathLibrary.BreakVector` (`self.K2_GetActorLocation`)))
  (bind (_returnvalue_x_3 _returnvalue_y_3 _returnvalue_z_2) (`KismetMathLibrary.BreakVector` (`self.K2_GetActorLocation`)))
  (bind (_returnvalue_x_4 _returnvalue_y_4 _returnvalue_z_3) (`KismetMathLibrary.BreakVector` (`self.K2_GetActorLocation`)))
  (bind (_returnvalue_x_5 _returnvalue_y_5 _returnvalue_z_4) (`KismetMathLibrary.BreakVector` (`self.K2_GetActorLocation`)))
  (bind (_returnvalue_x_6 _returnvalue_y_6 _returnvalue_z_5) (`KismetMathLibrary.BreakVector` (`self.K2_GetActorLocation`)))
  (bind (_returnvalue_x_7 _returnvalue_y_7 _returnvalue_z_6) (`KismetMathLibrary.BreakVector` (`self.K2_GetActorLocation`)))
  (bind (_returnvalue_x_8 _returnvalue_y_8) (`KismetMathLibrary.BreakVector` (`self.K2_GetActorLocation`)))
  (bind (_returnvalue_x_9 _returnvalue_y_9) (`KismetMathLibrary.BreakVector` (`self.K2_GetActorLocation`)))
  (bind _returnvalue_x_10 (`KismetMathLibrary.BreakVector` (`self.K2_GetActorLocation`)))
  (bind (_returnvalue_x_11 _returnvalue_y_10 _returnvalue_z_7) (`KismetMathLibrary.BreakVector` (`self.K2_GetActorLocation`)))
  (bind (_returnvalue_x_12 _returnvalue_y_11) (`KismetMathLibrary.BreakVector` (`self.K2_GetActorLocation`)))
  (bind (_returnvalue_x_13 _returnvalue_y_12 _returnvalue_z_8) (`KismetMathLibrary.BreakVector` (`self.K2_GetActorLocation`)))
  (bind (_returnvalue_x_14 _returnvalue_y_13) (`KismetMathLibrary.BreakVector` (`self.K2_GetActorLocation`)))
  (bind (_returnvalue_x_15 _returnvalue_y_14 _returnvalue_z_9) (`KismetMathLibrary.BreakVector` (`self.K2_GetActorLocation`)))
  (bind (_returnvalue_x_16 _returnvalue_y_15) (`KismetMathLibrary.BreakVector` (`self.K2_GetActorLocation`)))
  (bind (_returnvalue_x_17 _returnvalue_y_16) (`KismetMathLibrary.BreakVector` (`self.K2_GetActorLocation`)))
  (bind (_returnvalue_x_18 _returnvalue_y_17 _returnvalue_z_10) (`KismetMathLibrary.BreakVector` (`self.K2_GetActorLocation`)))
  (bind (_returnvalue_x_19 _returnvalue_y_18) (`KismetMathLibrary.BreakVector` (`self.K2_GetActorLocation`)))
  (bind (_returnvalue_x_20 _returnvalue_y_19) (`KismetMathLibrary.BreakVector` (`self.K2_GetActorLocation`)))
  (bind (_returnvalue_x_21 _returnvalue_y_20) (`KismetMathLibrary.BreakVector` (`self.K2_GetActorLocation`)))
  (bind (_returnvalue_x_22 _returnvalue_y_21) (`KismetMathLibrary.BreakVector` (`self.K2_GetActorLocation`)))
  (bind (_returnvalue_x_23 _returnvalue_y_22) (`KismetMathLibrary.BreakVector` (`self.K2_GetActorLocation`)))
  (bind (_returnvalue_x_24 _returnvalue_y_23) (`KismetMathLibrary.BreakVector` (`self.K2_GetActorLocation`)))
  (bind (_returnvalue_x_25 _returnvalue_y_24) (`KismetMathLibrary.BreakVector` (`self.K2_GetActorLocation`)))
  (bind _returnvalue (- _returnvalue_x (`self.EnemySpeedX`)))
  (bind _returnvalue_2 (- _returnvalue_x_4 (`self.EnemySpeedX`)))
  (bind _returnvalue_3 (- _returnvalue_x_6 (`self.EnemySpeedX`)))
  (if (`self.isRideOnDashEnemy`)
    (if (`self.isRidedOn`)
      (bind _asplayer_chara_bp (cast `/Game/BP/PlayerCharaBP` (`GameplayStatics.GetPlayerPawn` 0) :!label _label))
      (if (`self.CanMove`)
        (if (== (`self.EnemyType`) 0)
          ;[1 1 1] 0:横うねり
          (if (`self.IsLeft`)
            (`self.K2_SetActorLocation` (`KismetMathLibrary.MakeVector` _returnvalue_x_3 (+ (`self.EnemySpeedY`) _returnvalue_y_3) _returnvalue_z_2))
            (if (> _returnvalue_y_23 900.0)
              (`self.K2_SetActorLocation` (`KismetMathLibrary.MakeVector` _returnvalue _returnvalue_y _returnvalue_z))
              (if (> _returnvalue_y_22 1500.0)
                (set `self.IsLeft` false)))
            (else
              (`self.K2_SetActorLocation` (`KismetMathLibrary.MakeVector` _returnvalue_x_3 (- _returnvalue_y_3 (`self.EnemySpeedY`)) _returnvalue_z_2))
              (if (< _returnvalue_y_11 -900.0)
                (`self.K2_SetActorLocation` (`KismetMathLibrary.MakeVector` _returnvalue _returnvalue_y _returnvalue_z))
                (if (< _returnvalue_y_24 -1500.0)
                  (set `self.IsLeft` true)))))
          (elif (== (`self.EnemyType`) 1)
            ;[1 1 1] 1:斜めin
            (if (`self.IsLeft`)
              (`self.K2_SetActorLocation` (`KismetMathLibrary.MakeVector` (- _returnvalue_x_15 (`self.EnemySpeedX`)) (+ (`self.EnemySpeedY`) _returnvalue_y_14) _returnvalue_z_9))
              (if (> _returnvalue_y_16 (`self.RightDestroyPosY`))
                (`self.K2_DestroyActor`))
              (else
                (`self.K2_SetActorLocation` (`KismetMathLibrary.MakeVector` (- _returnvalue_x_15 (`self.EnemySpeedX`)) (- _returnvalue_y_14 (`self.EnemySpeedY`)) _returnvalue_z_9))
                (if (< _returnvalue_y_15 (`self.LeftDestroyPosY`))
                  (`self.K2_DestroyActor`))))
            (elif (== (`self.EnemyType`) 2)
              ;[1 1 1] 2:斜めin（逆）
              (if (`self.IsLeft`)
                (`self.K2_SetActorLocation` (`KismetMathLibrary.MakeVector` (+ (`self.EnemySpeedX`) _returnvalue_x_18) (+ (`self.EnemySpeedY`) _returnvalue_y_17) _returnvalue_z_10))
                (if (> _returnvalue_y_19 (`self.RightDestroyPosY`))
                  (`self.K2_DestroyActor`))
                (else
                  (`self.K2_SetActorLocation` (`KismetMathLibrary.MakeVector` (+ _returnvalue_x_18 (`self.EnemySpeedX`)) (- _returnvalue_y_17 (`self.EnemySpeedY`)) _returnvalue_z_10))
                  (if (< _returnvalue_y_18 (`self.LeftDestroyPosY`))
                    (`self.K2_DestroyActor`))))
              (elif (== (`self.EnemyType`) 3)
                ;[1 1 1] 3:横カット
                (if (`self.IsLeft`)
                  (`self.K2_SetActorLocation` (`KismetMathLibrary.MakeVector` _returnvalue_x_13 (+ (`self.EnemySpeedY`) _returnvalue_y_12) _returnvalue_z_8))
                  (if (> _returnvalue_y_9 (`self.RightDestroyPosY`))
                    (`self.K2_DestroyActor`))
                  (else
                    (`self.K2_SetActorLocation` (`KismetMathLibrary.MakeVector` _returnvalue_x_13 (- _returnvalue_y_12 (`self.EnemySpeedY`)) _returnvalue_z_8))
                    (if (< _returnvalue_y_8 (`self.LeftDestroyPosY`))
                      (`self.K2_DestroyActor`))))
                (elif (== (`self.EnemyType`) 4)
                  ;[1 1 1] 4:直角inout
                  (if (`self.IsLeft`)
                    (`self.K2_SetActorLocation` (`KismetMathLibrary.MakeVector` _returnvalue_2 (+ _returnvalue_y_4 (`self.EnemySpeedY`)) _returnvalue_z_3))
                    (if (== (`self.CurveCount`) 0)
                      (if (> _returnvalue_y_20 1500.0)
                        (`self.K2_SetActorRotation` (struct :`Yaw` 45.0))
                        (set `self.IsLeft` false)
                        (set `self.CurveCount` 1))
                      (elif (> _returnvalue_y_20 (`self.RightDestroyPosY`))
                        (`self.K2_DestroyActor`)))
                    (else
                      (`self.K2_SetActorLocation` (`KismetMathLibrary.MakeVector` _returnvalue_2 (- _returnvalue_y_4 (`self.EnemySpeedY`)) _returnvalue_z_3))
                      (if (== (`self.CurveCount`) 0)
                        (if (< _returnvalue_y_21 -1500.0)
                          (`self.K2_SetActorRotation` (struct :`Yaw` -45.0))
                          (set `self.IsLeft` true)
                          (set `self.CurveCount` 1))
                        (elif (< _returnvalue_y_21 (`self.LeftDestroyPosY`))
                          (`self.K2_DestroyActor`)))))
                  (elif (== (`self.EnemyType`) 5)
                    (bind _asplayer_chara_bp_2 (cast `/Game/BP/PlayerCharaBP` (`GameplayStatics.GetPlayerPawn` 0)))
                    ;[1 1 1] 5:直進in直角out
                    (if (`self.IsLeft`)
                      (bind _returnvalue_x_26 (`KismetMathLibrary.BreakVector` (`self.K2_GetActorLocation` _asplayer_chara_bp_2)))
                      (bind _returnvalue_4 (< (- _returnvalue_x_6 _returnvalue_x_26) (`self.CurveGap`)))
                      (if _returnvalue_4
                        (`self.K2_SetActorRotation` (struct :`Yaw` 90.0))
                        (`self.K2_SetActorLocation` (`KismetMathLibrary.MakeVector` _returnvalue_x_7 (- _returnvalue_y_7 (`self.EnemySpeedY`)) _returnvalue_z_6))
                        (if (< _returnvalue_y_2 (`self.LeftDestroyPosY`))
                          (`KismetSystemLibrary.PrintString` "Hello")
                          (`self.K2_DestroyActor`))
                        (else
                          (`self.K2_SetActorLocation` (`KismetMathLibrary.MakeVector` _returnvalue_3 _returnvalue_y_6 _returnvalue_z_5))))
                      (elif _returnvalue_4
                        (`self.K2_SetActorRotation` (struct :`Yaw` -90.0))
                        (`self.K2_SetActorLocation` (`KismetMathLibrary.MakeVector` _returnvalue_x_5 (+ _returnvalue_y_5 (`self.EnemySpeedY`)) _returnvalue_z_4))
                        (if (> _returnvalue_y_13 (`self.RightDestroyPosY`))
                          (`KismetSystemLibrary.PrintString` "Hello")
                          (`self.K2_DestroyActor`))
                        (else
                          (`self.K2_SetActorLocation` (`KismetMathLibrary.MakeVector` _returnvalue_3 _returnvalue_y_6 _returnvalue_z_5)))))))))))
        (else
          (bind _returnvalue_x_27 (`KismetMathLibrary.BreakVector` (`self.K2_GetActorLocation` _asplayer_chara_bp)))
          (if (< (- _returnvalue_x_10 _returnvalue_x_27) 10000.0)
            (set `self.CanMove` true)
            (else
              (`self.K2_SetActorLocation` (`KismetMathLibrary.MakeVector` (- _returnvalue_x_11 10.0) _returnvalue_y_10 _returnvalue_z_7))))))
      (else
        (`KismetSystemLibrary.PrintString` "Hit!!")
        (`self.K2_DestroyActor`)))
    (else
      (goto _label))))

(fn `UserConstructionScript`)