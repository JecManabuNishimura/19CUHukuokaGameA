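; Dash enemy that advances along X once the game starts, then charges at the player's position when close.
; It snapshots that position once within MaxDistance and lunges at twice player speed, dying near the target point.
; PlayerBullet hits reduce HP, and a kill grants dash energy.
; Any death awards score, kill count and capped dash energy, then fades two dynamic materials before destruction; rider-spawning logic is disconnected.
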(event `self.ReceiveActorBeginOverlap`
  (params (OtherActor :type "Actor Object Reference"))
  (if (`self.ActorHasTag` OtherActor "PlayerBullet")
    (`self.K2_DestroyActor` OtherActor)
    (set `self.HP` (- (`self.HP`) 1))
    (if (<= (`self.HP`) 0)
      (`PrimitiveComponent.SetCollisionEnabled` (`self.Box`) "NoCollision")
      (`/Engine/EditorBlueprintResources/StandardMacros.DoOnce` false
        (:`Completed`
          (bind _asplayer_chara_bp (cast `/Game/BP/PlayerCharaBP` (`GameplayStatics.GetPlayerPawn` 0)))
          (set `PlayerChara.DashEnergy` (+ (`PlayerChara.DashEnergy` _asplayer_chara_bp) (`PlayerChara.AddDashEnergy` _asplayer_chara_bp)) _asplayer_chara_bp)
          (set `self.isDead` true))))))

(event `self.ReceiveTick`
  (params (DeltaSeconds :type "Float (single-precision)"))
  (bind (_returnvalue_x _returnvalue_y _returnvalue_z) (`KismetMathLibrary.BreakVector` (`self.K2_GetActorLocation`)))
  (bind _returnvalue (- (`self.PlayerLocation`) (`self.K2_GetActorLocation`)))
  (if (`self.isDead`)
    (if (`self.IsScoreAdd`)
      ;[1 1 1] Material FadeOut(透明度を徐々に0までにする)
      (bind _output_get (set `self.CountTime` (+ (`self.CountTime`) (* DeltaSeconds (`self.DeadEffectDuration`)))))
      (`|ExecutionSequence`
        (:`then_0`
          (bind _returnvalue_2 (`PrimitiveComponent.CreateDynamicMaterialInstance` (`self.DashEnemy`) 0 "/Game/EnemyFBX/Dash_Enemy/Dash_Enemy.Dash_Enemy" "None"))
          (`MaterialInstanceDynamic.SetScalarParameterValue` _returnvalue_2 "FadeOut" (`KismetMathLibrary.Lerp` 1.0 0.0 _output_get)))
        (:`then_1`
          (bind _returnvalue_3 (`PrimitiveComponent.CreateDynamicMaterialInstance` (`self.DashEnemy`) 1 "/Game/EnemyFBX/Dash_Enemy/Dash_Enemy2.Dash_Enemy2" "None"))
          (bind _returnvalue_4 (`KismetMathLibrary.Lerp` 1.0 0.0 _output_get))
          (`MaterialInstanceDynamic.SetScalarParameterValue` _returnvalue_3 "FadeOut" _returnvalue_4))
        (:`then_2`
          (if (<= _returnvalue_4 0.0)
            (`self.K2_DestroyActor`))))
      (else
        (bind _asplayer_chara_bp (cast `/Game/BP/PlayerCharaBP` (`GameplayStatics.GetPlayerPawn` 0)))
        (set `PlayerChara.ScoreAnimStart` true _asplayer_chara_bp)
        (set `PlayerChara.CountShootEnemy` (+ (`PlayerChara.CountShootEnemy` _asplayer_chara_bp) 1) _asplayer_chara_bp)
        (set `PlayerChara.PlayerScore` (+ (`PlayerChara.PlayerScore` _asplayer_chara_bp) (`self.DashEnemyScore`)) _asplayer_chara_bp)
        (if (> (`PlayerChara.DashEnergyMax` _asplayer_chara_bp) (`PlayerChara.DashEnergy` _asplayer_chara_bp))
          (set `PlayerChara.DashEnergy` (+ (`PlayerChara.DashEnergy` _asplayer_chara_bp) (`PlayerChara.AddDashEnergy` _asplayer_chara_bp)) _asplayer_chara_bp))
        (set `self.IsScoreAdd` true)))
    (else
      (bind _asplayer_chara_bp_2 (cast `/Game/BP/PlayerCharaBP` (`GameplayStatics.GetPlayerPawn` 0)))
      (if (`PlayerChara.isStart` _asplayer_chara_bp_2)
        (if (`self.isCloseToPlayer`)
          (`self.K2_SetActorRotation` (`KismetMathLibrary.RLerp` (`self.K2_GetActorRotation`) (`KismetMathLibrary.FindLookAtRotation` (`self.PlayerLocation`) (`self.K2_GetActorLocation`)) 1.0))
          (`self.K2_SetActorLocation` (+ (`self.K2_GetActorLocation`) (* (`KismetMathLibrary.Normal` _returnvalue) (* (`PlayerChara.playerSpeed` _asplayer_chara_bp_2) 2.0))))
          (if (and (<= (`KismetMathLibrary.VSize` _returnvalue) 100.0) (> (.x _returnvalue) 0.0))
            (set `self.isDead` true))
          (else
            (bind _returnvalue_x_2 (`KismetMathLibrary.BreakVector` (- (`self.K2_GetActorLocation`) (`self.K2_GetActorLocation` _asplayer_chara_bp_2))))
            (if (> _returnvalue_x_2 (`self.MaxDistance`))
              (`self.K2_SetActorLocation` (`KismetMathLibrary.MakeVector` (+ _returnvalue_x (`self.MoveSpeed`)) _returnvalue_y _returnvalue_z))
              (set `self.isCloseToPlayer` false)
              (else
                (set `self.isCloseToPlayer` true)
                (bind _asplayer_chara_bp_3 (cast `/Game/BP/PlayerCharaBP` (`GameplayStatics.GetPlayerPawn` 0)))
                (set `self.PlayerLocation` (`self.K2_GetActorLocation` _asplayer_chara_bp_3))))))))))

(event `self.Box.OnComponentBeginOverlap`
  (params (OverlappedComponent :type "PrimitiveComponent Object Reference") (OtherActor :type "Actor Object Reference") (OtherComp :type "PrimitiveComponent Object Reference") (OtherBodyIndex :type Integer) (bFromSweep :type Boolean) (SweepResult :type "HitResult Structure (by ref)")))

(event `self.ReceiveBeginPlay`)

(fn `UserConstructionScript`)