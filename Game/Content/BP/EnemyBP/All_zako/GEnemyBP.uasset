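; General small-fry enemy for a shooter that moves in one of several EnemyType patterns (weaving, diagonal, side cut, turning, side-to-side).
; Tick moves it once the player has started and is near, destroys it when left behind or off-side, and can tie it to a DashEnemy ride.
; PlayerBullet overlaps drain HP; death adds score, kill count and dash energy to PlayerCharaBP, then fades the mesh via a dynamic material before destroying it.
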(event `self.ReceiveBeginPlay`
  (bind (_returnvalue_x _returnvalue_y) (`KismetMathLibrary.BreakVector` (`self.K2_GetActorLocation`)))
  (if (== (`self.Direction`) 0)
    (set `self.EnemySpeedX` 50.0)
    (else
      (set `self.EnemySpeedX` -50.0)))
  (if (< _returnvalue_y 0.0)
    (set `self.IsLeft` true)
    (else
      (set `self.IsLeft` false)))
  (if (== (`self.EnemyType`) 4)
    (if (`self.IsLeft`)
      (`self.K2_SetActorRotation` (struct :`Yaw` -45.0))
      (else
        (`self.K2_SetActorRotation` (struct :`Yaw` 45.0))))))

(event `self.ReceiveActorBeginOverlap`
  (params (OtherActor :type "Actor Object Reference"))
  (if (`self.ActorHasTag` OtherActor "PlayerBullet")
    (`self.K2_DestroyActor` OtherActor)
    (set `self.HP` (- (`self.HP`) 1))
    (if (<= (`self.HP`) 0)
      (`PrimitiveComponent.SetCollisionEnabled` (`self.Box`) "NoCollision")
      (`/Engine/EditorBlueprintResources/StandardMacros.DoOnce` false
        (:`Completed`
          (bind _asplayer_chara_bp (cast `/Game/BP/PlayerCharaBP` (`GameplayStatics.GetPlayerPawn` 0)))
          (set `PlayerChara.ScoreAnimStart` true _asplayer_chara_bp)
          (set `PlayerChara.PlayerScore` (+ (`PlayerChara.PlayerScore` _asplayer_chara_bp) (`self.GeneralEnemyScore`)) _asplayer_chara_bp)
          (set `PlayerChara.CountShootEnemy` (+ (`PlayerChara.CountShootEnemy` _asplayer_chara_bp) 1) _asplayer_chara_bp)
          (if (> (`PlayerChara.DashEnergyMax` _asplayer_chara_bp) (`PlayerChara.DashEnergy` _asplayer_chara_bp))
            (set `PlayerChara.DashEnergy` (+ (`PlayerChara.DashEnergy` _asplayer_chara_bp) (`PlayerChara.AddDashEnergy` _asplayer_chara_bp)) _asplayer_chara_bp))
          (set `self.IsDead` true))))))

(event `self.ReceiveTick`
  (params (DeltaSeconds :type "Float (single-precision)"))
  (bind (_returnvalue_x _returnvalue_y _returnvalue_z) (`KismetMathLibrary.BreakVector` (`self.K2_GetActorLocation`)))
  (bind (_returnvalue_x_2 _returnvalue_y_2) (`KismetMathLibrary.BreakVector` (`self.K2_GetActorLocation`)))
  (bind (_returnvalue_x_3 _returnvalue_y_3 _returnvalue_z_2) (`KismetMathLibrary.BreakVector` (`self.K2_GetActorLocation`)))
  (bind (_returnvalue_x_4 _returnvalue_y_4 _returnvalue_z_3) (`KismetMathLibrary.BreakVector` (`self.K2_GetActorLocation`)))
  (bind _returnvalue_x_5 (`KismetMathLibrary.BreakVector` (`self.K2_GetActorLocation`)))
  (bind (_returnvalue_x_6 _returnvalue_y_5 _returnvalue_z_4) (`KismetMathLibrary.BreakVector` (`self.K2_GetActorLocation`)))
  (bind (_returnvalue_x_7 _returnvalue_y_6 _returnvalue_z_5) (`KismetMathLibrary.BreakVector` (`self.K2_GetActorLocation`)))
  (bind (_returnvalue_x_8 _returnvalue_y_7 _returnvalue_z_6) (`KismetMathLibrary.BreakVector` (`self.K2_GetActorLocation`)))
  (bind (_returnvalue_x_9 _returnvalue_y_8) (`KismetMathLibrary.BreakVector` (`self.K2_GetActorLocation`)))
  (bind (_returnvalue_x_10 _returnvalue_y_9) (`KismetMathLibrary.BreakVector` (`self.K2_GetActorLocation`)))
  (bind (_returnvalue_x_11 _returnvalue_y_10 _returnvalue_z_7) (`KismetMathLibrary.BreakVector` (`self.K2_GetActorLocation`)))
  (bind (_returnvalue_x_12 _returnvalue_y_11 _returnvalue_z_8) (`KismetMathLibrary.BreakVector` (`self.K2_GetActorLocation`)))
  (bind (_returnvalue_x_13 _returnvalue_y_12) (`KismetMathLibrary.BreakVector` (`self.K2_GetActorLocation`)))
  (bind (_returnvalue_x_14 _returnvalue_y_13) (`KismetMathLibrary.BreakVector` (`self.K2_GetActorLocation`)))
  (bind (_returnvalue_x_15 _returnvalue_y_14) (`KismetMathLibrary.BreakVector` (`self.K2_GetActorLocation`)))
  (bind _returnvalue_x_16 (`KismetMathLibrary.BreakVector` (`self.K2_GetActorLocation`)))
  (bind (_returnvalue_x_17 _returnvalue_y_15) (`KismetMathLibrary.BreakVector` (`self.K2_GetActorLocation`)))
  (bind (_returnvalue_x_18 _returnvalue_y_16 _returnvalue_z_9) (`KismetMathLibrary.BreakVector` (`self.K2_GetActorLocation`)))
  (bind (_returnvalue_x_19 _returnvalue_y_17) (`KismetMathLibrary.BreakVector` (`self.K2_GetActorLocation`)))
  (bind (_returnvalue_x_20 _returnvalue_y_18 _returnvalue_z_10) (`KismetMathLibrary.BreakVector` (`self.K2_GetActorLocation`)))
  (bind (_returnvalue_x_21 _returnvalue_y_19) (`KismetMathLibrary.BreakVector` (`self.K2_GetActorLocation`)))
  (bind (_returnvalue_x_22 _returnvalue_y_20) (`KismetMathLibrary.BreakVector` (`self.K2_GetActorLocation`)))
  (bind (_returnvalue_x_23 _returnvalue_y_21 _returnvalue_z_11) (`KismetMathLibrary.BreakVector` (`self.K2_GetActorLocation`)))
  (bind (_returnvalue_x_24 _returnvalue_y_22) (`KismetMathLibrary.BreakVector` (`self.K2_GetActorLocation`)))
  (bind (_returnvalue_x_25 _returnvalue_y_23) (`KismetMathLibrary.BreakVector` (`self.K2_GetActorLocation`)))
  (bind (_returnvalue_x_26 _returnvalue_y_24) (`KismetMathLibrary.BreakVector` (`self.K2_GetActorLocation`)))
  (bind (_returnvalue_x_27 _returnvalue_y_25) (`KismetMathLibrary.BreakVector` (`self.K2_GetActorLocation`)))
  (bind (_returnvalue_x_28 _returnvalue_y_26) (`KismetMathLibrary.BreakVector` (`self.K2_GetActorLocation`)))
  (bind (_returnvalue_x_29 _returnvalue_y_27) (`KismetMathLibrary.BreakVector` (`self.K2_GetActorLocation`)))
  (bind (_returnvalue_x_30 _returnvalue_y_28) (`KismetMathLibrary.BreakVector` (`self.K2_GetActorLocation`)))
  (bind _returnvalue (- _returnvalue_x (`self.EnemySpeedX`)))
  (bind _returnvalue_2 (- _returnvalue_x_4 (`self.EnemySpeedX`)))
  (bind _returnvalue_3 (- _returnvalue_x_11 (`self.EnemySpeedX`)))
  (if (`self.IsDead`)
    ;[1 1 1] Material FadeOut(透明度を徐々に0までにする)
    (`GameplayStatics.SpawnEmitterAttached` "/Game/Effect/Damage.Damage" (`self.RootComponent`))
    (bind _output_get (set `self.CountTime` (+ (`self.CountTime`) (* DeltaSeconds (`self.DeadEffectDuration`)))))
    (`|ExecutionSequence`
      (:`then_1`
        (bind _returnvalue_4 (`PrimitiveComponent.CreateDynamicMaterialInstance` (`self.StaticMesh`) 0 "/Game/EnemyFBX/Enemy/EnemyMat.EnemyMat" "None"))
        (bind _returnvalue_5 (`KismetMathLibrary.Lerp` 1.0 0.0 _output_get))
        (`MaterialInstanceDynamic.SetScalarParameterValue` _returnvalue_4 "FadeOut" _returnvalue_5))
      (:`then_2`
        (if (<= _returnvalue_5 0.0)
          (`self.K2_DestroyActor`))))
    (elif (`self.isRideOnDashEnemy`)
      (`self.K2_SetActorLocation` (`KismetMathLibrary.MakeVector` _returnvalue_x_15 _returnvalue_y_14 500.0))
      (if (`self.isRidedOn`)
        (bind _asplayer_chara_bp (cast `/Game/BP/PlayerCharaBP` (`GameplayStatics.GetPlayerPawn` 0) :!label _label))
        (if (`PlayerChara.isStart` _asplayer_chara_bp)
          (if (`PlayerChara.isDead` _asplayer_chara_bp)
            _
            (elif (not (`PlayerChara.isGoal` _asplayer_chara_bp))
              (bind _returnvalue_x_31 (`KismetMathLibrary.BreakVector` (`self.K2_GetActorLocation` _asplayer_chara_bp)))
              (if (< (+ _returnvalue_x_5 (`self.DistanceToPlayer`)) _returnvalue_x_31)
                (`self.K2_DestroyActor`)
                (elif (`self.CanMove`)
                  (if (== (`self.EnemyType`) 0)
                    ;[1 1 1] 0:横うねり
                    (if (`self.IsLeft`)
                      (`self.K2_SetActorLocation` (`KismetMathLibrary.MakeVector` _returnvalue_x_3 (+ (`self.EnemySpeedY`) _returnvalue_y_3) _returnvalue_z_2))
                      (if (> _returnvalue_y_27 3500.0)
                        (`self.K2_SetActorLocation` (`KismetMathLibrary.MakeVector` _returnvalue _returnvalue_y _returnvalue_z))
                        (if (> _returnvalue_y_26 5000.0)
                          (set `self.IsLeft` false)))
                      (else
                        (`self.K2_SetActorLocation` (`KismetMathLibrary.MakeVector` _returnvalue_x_3 (- _returnvalue_y_3 (`self.EnemySpeedY`)) _returnvalue_z_2))
                        (if (< _returnvalue_y_15 -3500.0)
                          (`self.K2_SetActorLocation` (`KismetMathLibrary.MakeVector` _returnvalue _returnvalue_y _returnvalue_z))
                          (if (< _returnvalue_y_28 -5000.0)
                            (set `self.IsLeft` true)))))
                    (elif (== (`self.EnemyType`) 1)
                      ;[1 1 1] 1:斜めin
                      (if (`self.IsLeft`)
                        (`self.K2_SetActorLocation` (`KismetMathLibrary.MakeVector` (- _returnvalue_x_20 (`self.EnemySpeedX`)) (+ (`self.EnemySpeedY`) _returnvalue_y_18) _returnvalue_z_10))
                        (if (> _returnvalue_y_20 (`self.RightDestroyPosY`))
                          (`self.K2_DestroyActor`))
                        (else
                          (`self.K2_SetActorLocation` (`KismetMathLibrary.MakeVector` (- _returnvalue_x_20 (`self.EnemySpeedX`)) (- _returnvalue_y_18 (`self.EnemySpeedY`)) _returnvalue_z_10))
                          (if (< _returnvalue_y_19 (`self.LeftDestroyPosY`))
                            (`self.K2_DestroyActor`))))
                      (elif (== (`self.EnemyType`) 2)
                        ;[1 1 1] 2:斜めin（逆）
                        (if (`self.IsLeft`)
                          (`self.K2_SetActorLocation` (`KismetMathLibrary.MakeVector` (+ (`self.EnemySpeedX`) _returnvalue_x_23) (+ (`self.EnemySpeedY`) _returnvalue_y_21) _returnvalue_z_11))
                          (if (> _returnvalue_y_23 (`self.RightDestroyPosY`))
                            (`self.K2_DestroyActor`))
                          (else
                            (`self.K2_SetActorLocation` (`KismetMathLibrary.MakeVector` (+ _returnvalue_x_23 (`self.EnemySpeedX`)) (- _returnvalue_y_21 (`self.EnemySpeedY`)) _returnvalue_z_11))
                            (if (< _returnvalue_y_22 (`self.LeftDestroyPosY`))
                              (`self.K2_DestroyActor`))))
                        (elif (== (`self.EnemyType`) 3)
                          ;[1 1 1] 3:横カット
                          (if (`self.IsLeft`)
                            (`self.K2_SetActorLocation` (`KismetMathLibrary.MakeVector` _returnvalue_x_18 (+ (`self.EnemySpeedY`) _returnvalue_y_16) _returnvalue_z_9))
                            (if (> _returnvalue_y_9 (`self.RightDestroyPosY`))
                              (`self.K2_DestroyActor`))
                            (else
                              (`self.K2_SetActorLocation` (`KismetMathLibrary.MakeVector` _returnvalue_x_18 (- _returnvalue_y_16 (`self.EnemySpeedY`)) _returnvalue_z_9))
                              (if (< _returnvalue_y_8 (`self.LeftDestroyPosY`))
                                (`self.K2_DestroyActor`))))
                          (elif (== (`self.EnemyType`) 4)
                            ;[1 1 1] 4:直角inout
                            (if (`self.IsLeft`)
                              (`self.K2_SetActorLocation` (`KismetMathLibrary.MakeVector` _returnvalue_2 (+ _returnvalue_y_4 (`self.EnemySpeedY`)) _returnvalue_z_3))
                              (if (== (`self.CurveCount`) 0)
                                (if (> _returnvalue_y_24 5000.0)
                                  (`self.K2_SetActorRotation` (struct :`Yaw` 45.0))
                                  (set `self.IsLeft` false)
                                  (set `self.CurveCount` 1))
                                (elif (> _returnvalue_y_24 (`self.RightDestroyPosY`))
                                  (`self.K2_DestroyActor`)))
                              (else
                                (`self.K2_SetActorLocation` (`KismetMathLibrary.MakeVector` _returnvalue_2 (- _returnvalue_y_4 (`self.EnemySpeedY`)) _returnvalue_z_3))
                                (if (== (`self.CurveCount`) 0)
                                  (if (< _returnvalue_y_25 -5000.0)
                                    (`self.K2_SetActorRotation` (struct :`Yaw` -45.0))
                                    (set `self.IsLeft` true)
                                    (set `self.CurveCount` 1))
                                  (elif (< _returnvalue_y_25 (`self.LeftDestroyPosY`))
                                    (`self.K2_DestroyActor`)))))
                            (elif (== (`self.EnemyType`) 5)
                              (bind _asplayer_chara_bp_2 (cast `/Game/BP/PlayerCharaBP` (`GameplayStatics.GetPlayerPawn` 0)))
                              ;[1 1 1] 5:直進in直角out
                              (if (`self.IsLeft`)
                                (bind _returnvalue_x_32 (`KismetMathLibrary.BreakVector` (`self.K2_GetActorLocation` _asplayer_chara_bp_2)))
                                (bind _returnvalue_6 (< (- _returnvalue_x_11 _returnvalue_x_32) (`self.CurveGap`)))
                                (if _returnvalue_6
                                  (`self.K2_SetActorRotation` (struct :`Yaw` 90.0))
                                  (`self.K2_SetActorLocation` (`KismetMathLibrary.MakeVector` _returnvalue_x_8 (- _returnvalue_y_7 (`self.EnemySpeedY`)) _returnvalue_z_6))
                                  (if (< _returnvalue_y_2 (`self.LeftDestroyPosY`))
                                    (`self.K2_DestroyActor`))
                                  (else
                                    (`self.K2_SetActorLocation` (`KismetMathLibrary.MakeVector` _returnvalue_3 _returnvalue_y_10 _returnvalue_z_7))))
                                (elif _returnvalue_6
                                  (`self.K2_SetActorRotation` (struct :`Yaw` -90.0))
                                  (`self.K2_SetActorLocation` (`KismetMathLibrary.MakeVector` _returnvalue_x_6 (+ _returnvalue_y_5 (`self.EnemySpeedY`)) _returnvalue_z_4))
                                  (if (> _returnvalue_y_17 (`self.RightDestroyPosY`))
                                    (`self.K2_DestroyActor`))
                                  (else
                                    (`self.K2_SetActorLocation` (`KismetMathLibrary.MakeVector` _returnvalue_3 _returnvalue_y_10 _returnvalue_z_7)))))
                              (elif (== (`self.EnemyType`) 6)
                                (if (`self.IsLeft`)
                                  (if (> _returnvalue_y_12 (`self.YokoPosLeft`))
                                    (`self.K2_SetActorLocation` (`KismetMathLibrary.MakeVector` _returnvalue_x_7 (- _returnvalue_y_6 (`self.EnemySpeedY`)) _returnvalue_z_5))
                                    (else
                                      (set `self.IsLeft` false)))
                                  (elif (< _returnvalue_y_13 (+ (`self.YokoPosLeft`) (`self.YokoPosRight`)))
                                    (`self.K2_SetActorLocation` (`KismetMathLibrary.MakeVector` _returnvalue_x_12 (+ _returnvalue_y_11 (`self.EnemySpeedY`)) _returnvalue_z_8))
                                    (else
                                      (set `self.IsLeft` true)))))))))))
                  (else
                    (bind _returnvalue_x_33 (`KismetMathLibrary.BreakVector` (`self.K2_GetActorLocation` _asplayer_chara_bp)))
                    (if (< (- _returnvalue_x_16 _returnvalue_x_33) 100000.0)
                      (if (`PlayerChara.isStart` _asplayer_chara_bp)
                        (set `self.CanMove` true)))))))))
        (else
          (`self.K2_DestroyActor`)))
      (else
        (goto _label)))))

(fn `UserConstructionScript`)