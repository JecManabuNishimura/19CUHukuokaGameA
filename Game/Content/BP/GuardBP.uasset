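; GuardBP is a guard actor that stays in front of the player character and reacts to enemy bullets.
; Each Tick repositions it from the PlayerCharaBP pawn's location at a fixed world-axis X and Z offset, independent of facing.
; Overlapping an actor tagged EnemyBullet spawns the Reflect_P particle and prints debug text, leaving the bullet untouched.
; A disconnected timer that periodically fires the same effect remains from bullet-reflect testing.
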(event `self.ReceiveActorBeginOverlap`
  (params (OtherActor :type "Actor Object Reference"))
  (if (`self.ActorHasTag` OtherActor "EnemyBullet")
    (`GameplayStatics.SpawnEmitterAtLocation` "/Game/Effect/Reflect_P.Reflect_P" (`self.K2_GetActorLocation`))
    (`KismetSystemLibrary.PrintString` "Hello")))

(event `self.ReceiveTick`
  (params (DeltaSeconds :type "Float (single-precision)"))
  (bind _asplayer_chara_bp (cast `/Game/BP/PlayerCharaBP` (`GameplayStatics.GetPlayerPawn` 0)))
  (bind (_returnvalue_x _returnvalue_y _returnvalue_z) (`KismetMathLibrary.BreakVector` (`self.K2_GetActorLocation` _asplayer_chara_bp)))
  (`self.K2_SetActorRelativeLocation` (`KismetMathLibrary.MakeVector` (+ _returnvalue_x 500.0) _returnvalue_y (+ _returnvalue_z 50.0))))

(fn `UserConstructionScript`)