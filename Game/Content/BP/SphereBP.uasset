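; SphereBP is a sphere actor that follows the player and shows a spark effect when enemy bullets touch it.
; It enlarges itself on BeginPlay and copies the PlayerCharaBP location to its relative location every Tick.
; Overlaps with tagged EnemyBulletBP actors spawn a Spark emitter on the player's root at a fixed offset, not the impact point.
; A timed bullet-reflect particle test remains disconnected and never runs.
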(event `self.ReceiveBeginPlay`
  (`self.SetActorScale3D` (3.0 3.0 3.0)))

(event `self.ReceiveTick`
  (params (DeltaSeconds :type "Float (single-precision)"))
  (bind _asplayer_chara_bp (cast `/Game/BP/PlayerCharaBP` (`GameplayStatics.GetPlayerPawn` 0)))
  (bind (_returnvalue_x _returnvalue_y _returnvalue_z) (`KismetMathLibrary.BreakVector` (`self.K2_GetActorLocation` _asplayer_chara_bp)))
  (`self.K2_SetActorRelativeLocation` (`KismetMathLibrary.MakeVector` _returnvalue_x _returnvalue_y _returnvalue_z)))

(event `self.Sphere.OnComponentBeginOverlap`
  (params (OverlappedComponent :type "PrimitiveComponent Object Reference") (OtherActor :type "Actor Object Reference") (OtherComp :type "PrimitiveComponent Object Reference") (OtherBodyIndex :type Integer) (bFromSweep :type Boolean) (SweepResult :type "HitResult Structure (by ref)"))
  ;[1 1 1] 敵弾当たりのエフェクト
  (if (`self.ActorHasTag` OtherActor "EnemyBullet")
    (bind _asplayer_chara_bp (cast `/Game/BP/PlayerCharaBP` (`GameplayStatics.GetPlayerPawn` 0)))
    (bind _asenemy_bullet_bp (cast `/Game/Bullet/EnemyBulletBP` OtherActor))
    (`GameplayStatics.SpawnEmitterAttached` "/Game/Effect/SphereShield/spark.spark" (`Actor.RootComponent` _asplayer_chara_bp) "None" (1200.0 0.0 0.0) (struct :`Yaw` 180.0))))

(fn `UserConstructionScript`)