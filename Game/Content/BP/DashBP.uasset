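; DashBP is an actor that shadows the player character, likely as the visual for a dash.
; Each Tick it casts the player pawn to PlayerCharaBP and copies that pawn's location and rotation, pitched down 90 degrees, while applying its own ActorSize scale.
; It stops updating while the player is dead and destroys itself once the player's IsGoal flag is set.
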(event `self.ReceiveTick`
  (params (DeltaSeconds :type "Float (single-precision)"))
  (bind _asplayer_chara_bp (cast `/Game/BP/PlayerCharaBP` (`GameplayStatics.GetPlayerPawn` 0)))
  (if (`PlayerChara.isGoal` _asplayer_chara_bp)
    (`self.K2_DestroyActor`)
    (elif (not (`PlayerChara.isDead` _asplayer_chara_bp))
      (bind _returnvalue (`self.GetTransform` _asplayer_chara_bp))
      (`self.K2_SetActorTransform` (`KismetMathLibrary.MakeTransform` (.location _returnvalue) (`KismetMathLibrary.MakeRotator` (.roll (.rotation _returnvalue)) (+ (.pitch (.rotation _returnvalue)) -90.0) (.yaw (.rotation _returnvalue))) (`self.ActorSize`))))))

(fn `UserConstructionScript`)