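; Tutorial screen Blueprint that handles the key input for leaving to another level.
; BeginPlay pauses the Cancel and Decide audio, then Enter unpauses Decide and opens Loading, while Space unpauses Cancel and opens PlayerInputName.
; Each key has its own DoOnce, sets InsFlag on BP_MyInstance, and waits briefly before the level change so the sound can be heard.
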(event `self.ReceiveBeginPlay`
  (`AudioComponent.SetPaused` (`self.Cancel`) true)
  (`AudioComponent.SetPaused` (`self.Decide`) true))

(event `Key|Enter`
  (params (Key :type "Key Structure"))
  (:`Pressed`
    (`/Engine/EditorBlueprintResources/StandardMacros.DoOnce` false
      (:`Completed`
        (`AudioComponent.SetPaused` (`self.Decide`) false)
        (bind _asbp_my_instance (cast `/Game/BP/PlayerData/BP_MyInstance` (`GameplayStatics.GetGameInstance`)))
        (set `/Game/BP/PlayerData/BP_MyInstance.InsFlag` true _asbp_my_instance)
        (`KismetSystemLibrary.Delay` 1.0)
        (`GameplayStatics.OpenLevel` "Loading")))))

(event `Key|SpaceBar`
  (params (Key :type "Key Structure"))
  (:`Pressed`
    (`/Engine/EditorBlueprintResources/StandardMacros.DoOnce` false
      (:`Completed`
        (`AudioComponent.SetPaused` (`self.Cancel`) false)
        (bind _asbp_my_instance (cast `/Game/BP/PlayerData/BP_MyInstance` (`GameplayStatics.GetGameInstance`)))
        (set `/Game/BP/PlayerData/BP_MyInstance.InsFlag` true _asbp_my_instance)
        (`KismetSystemLibrary.Delay` 1.0)
        (`GameplayStatics.OpenLevel` "PlayerInputName")))))

(fn `UserConstructionScript`)