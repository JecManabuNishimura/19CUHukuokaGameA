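; BP_Box is an effect test actor that feeds a cube's transform to materials and slowly sinks during play.
; Its Construction Script writes the Cube's world location and scale into the PC_Data parameter collection as Position1 and Bounds.
; Tick moves the actor down by a fixed, frame-rate-dependent step without sweeping.
; Tick does not update the collection, so the published values do not follow this movement.
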(event `self.ReceiveTick`
  (params (DeltaSeconds :type "Float (single-precision)"))
  (`self.K2_SetActorLocation` (+ (`self.K2_GetActorLocation`) (0.0 0.0 -0.1))))

(fn `UserConstructionScript`
  (bind _cube (`self.Cube`))
  (`KismetMaterialLibrary.SetVectorParameterValue` "/Game/Effect/Try/PC_Data.PC_Data" "Position1" (`KismetMathLibrary.Conv_VectorToLinearColor` (`SceneComponent.K2_GetComponentLocation` _cube)))
  (`KismetMaterialLibrary.SetVectorParameterValue` "/Game/Effect/Try/PC_Data.PC_Data" "Bounds" (`KismetMathLibrary.Conv_VectorToLinearColor` (`SceneComponent.K2_GetComponentScale` _cube))))