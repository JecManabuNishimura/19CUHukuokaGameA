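; RingBP is a map object that lays out a grid of instanced ring meshes at construction and spins them every tick.
; Tick pitches alternate instances in opposite directions by PitchPerSecond, negating the pitch when it would pass ±90 degrees.
; It also removes instances once the player is 30000 units past them on X, flipping the DivideNum parity on each removal as indices shift.
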(event `self.ReceiveTick`
  (params (DeltaSeconds :type "Float (single-precision)"))
  (bind _instancedstaticmesh (`self.InstancedStaticMesh`))
  (bind _instancedstaticmesh_2 (`self.InstancedStaticMesh`))
  (bind _returnvalue_x (`KismetMathLibrary.BreakVector` (`self.K2_GetActorLocation` (`GameplayStatics.GetPlayerPawn` 0))))
  (for _index (range (`InstancedStaticMeshComponent.GetInstanceCount` _instancedstaticmesh_2))
    (if (>= (- _returnvalue_x (.x (.location (`InstancedStaticMeshComponent.GetInstanceTransform` _instancedstaticmesh_2 _index true)))) 30000.0)
      (`InstancedStaticMeshComponent.RemoveInstance` (`self.InstancedStaticMesh`) _index)
      (`/Engine/EditorBlueprintResources/StandardMacros.FlipFlop`
        (:`A`
          (set `self.divideNum` 1))
        (:`B`
          (set `self.divideNum` 0)))))
  (for _index_2 (range (+ (`InstancedStaticMeshComponent.GetInstanceCount` _instancedstaticmesh) 1))
    (if (== (mod _index_2 2) (`self.divideNum`))
      (set `self.direction` 1.0)
      (else
        (set `self.direction` -1.0)))
    (bind _outinstancetransform (`InstancedStaticMeshComponent.GetInstanceTransform` _instancedstaticmesh _index_2 false))
    (bind _returnvalue (+ (* (* DeltaSeconds (`self.Pitch Per Second`)) (`self.direction`)) (.pitch (.rotation _outinstancetransform))))
    (if (or (> _returnvalue 90.0) (< _returnvalue -90.0))
      (set `self.90Correction` -1.0)
      (else
        (set `self.90Correction` 1.0)))
    (`InstancedStaticMeshComponent.UpdateInstanceTransform` _instancedstaticmesh _index_2 (`KismetMathLibrary.MakeTransform` (.location _outinstancetransform) (`KismetMathLibrary.MakeRotator` 0.0 (* (`self.90Correction`) _returnvalue)) (.scale _outinstancetransform)) false true false)))

(fn `UserConstructionScript`
  (for _index (range (+ (`self.X`) 1))
    (for _index_2 (range (+ (`self.Y`) 1))
      (`InstancedStaticMeshComponent.AddInstance` (`self.InstancedStaticMesh`) (`KismetMathLibrary.Conv_VectorToTransform` (`KismetMathLibrary.MakeVector` (* _index (.x (`self.Vector`))) (* _index_2 (.y (`self.Vector`))) (.z (`self.Vector`))))))))