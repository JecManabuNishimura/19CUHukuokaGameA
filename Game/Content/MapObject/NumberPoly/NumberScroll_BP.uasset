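; NumberScroll_BP is a map prop whose Plane shows scrolling number characters, configured entirely in the construction script with no runtime logic.
; It derives a signed scroll speed from the direction flag, optionally dividing it by the actor's X/Y scale ratio to correct for stretching.
; That speed and a fixed or randomized texture sampling offset are written to the Plane's Custom Primitive Data, letting instances vary through per-primitive values.
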(fn `UserConstructionScript`
  (locals (multipleNum :type "Float (double-precision)") (speed :type "Float (double-precision)") (correctSpeed :type "Float (double-precision)") (texcoord_X :type "Float (double-precision)") (texcoord_Y :type "Float (double-precision)"))
  (bind _returnvalue (`self.GetTransform`))
  (bind _plane (`self.Plane`))
  (if (`self.isRight`)
    (set `local.multipleNum` 1.0)
    (else
      (set `local.multipleNum` -1.0)))
  (bind _output_get (set `local.speed` (* (`self.CharScrollSpeed`) (`local.multipleNum`))))
  (if (`self.isSpeedCorrection`)
    (set `local.correctSpeed` (/ _output_get (/ (.x (.scale _returnvalue)) (.y (.scale _returnvalue)))))
    (else
      (set `local.correctSpeed` _output_get)))
  (`PrimitiveComponent.SetCustomPrimitiveDataFloat` _plane 0 (`local.correctSpeed`))
  (if (`self.SetTexSampleRandom`)
    (set `local.texcoord_X` (`KismetMathLibrary.RandomFloatInRange` 0.0 1.0))
    (else
      (set `local.texcoord_X` (`self.TexSampling_X`))))
  (`PrimitiveComponent.SetCustomPrimitiveDataFloat` _plane 1 (`local.texcoord_X`))
  (if (`self.SetTexSampleRandom`)
    (set `local.texcoord_Y` (`KismetMathLibrary.RandomFloatInRange` 0.0 1.0))
    (else
      (set `local.texcoord_Y` (`self.TexSampling_Y`))))
  (`PrimitiveComponent.SetCustomPrimitiveDataFloat` _plane 2 (`local.texcoord_Y`)))