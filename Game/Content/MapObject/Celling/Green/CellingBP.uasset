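; CellingBP is a ceiling map object that builds a tiled grid from a single instanced static mesh.
; Its construction script runs nested loops over X and Y and adds one instance per cell, with both end indices included.
; The Margine vector sets the spacing along X and Y, while its Z gives every instance the same height offset.
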(fn `UserConstructionScript`
  (for _index (range (+ (`self.X`) 1))
    (for _index_2 (range (+ (`self.Y`) 1))
      (`InstancedStaticMeshComponent.AddInstance` (`self.InstancedStaticMesh`) (`KismetMathLibrary.Conv_VectorToTransform` (`KismetMathLibrary.MakeVector` (* _index (.x (`self.Margine`))) (* _index_2 (.y (`self.Margine`))) (.z (`self.Margine`))))))))