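; Tube map object that builds a grid of static meshes and removes itself once the player has left it behind.
; The Construction Script fills an InstancedStaticMesh with instances across inclusive X and Y counts, spaced by the Vector variable, whose Z sets a constant height.
; Each Tick it compares X positions with the PlayerCharaBP pawn and destroys itself when the player is far enough ahead along +X.
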(event `self.ReceiveTick`
  (params (DeltaSeconds :type "Float (single-precision)"))
  (bind _returnvalue_x (`KismetMathLibrary.BreakVector` (`self.K2_GetActorLocation`)))
  (bind _asplayer_chara_bp (cast `/Game/BP/PlayerCharaBP` (`GameplayStatics.GetPlayerPawn` 0)))
  (bind _returnvalue_x_2 (`KismetMathLibrary.BreakVector` (`self.K2_GetActorLocation` _asplayer_chara_bp)))
  (if (>= (- _returnvalue_x_2 _returnvalue_x) 30000.0)
    (`self.K2_DestroyActor`)))

(fn `UserConstructionScript`
  (for _index (range (+ (`self.X`) 1))
    (for _index_2 (range (+ (`self.Y`) 1))
      (`InstancedStaticMeshComponent.AddInstance` (`self.InstancedStaticMesh`) (`KismetMathLibrary.Conv_VectorToTransform` (`KismetMathLibrary.MakeVector` (* _index (.x (`self.Vector`))) (* _index_2 (.y (`self.Vector`))) (.z (`self.Vector`))))))))